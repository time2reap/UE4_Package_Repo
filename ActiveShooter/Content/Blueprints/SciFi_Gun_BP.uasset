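; VR paintball gun Blueprint that fires colored projectiles from limited ammo and returns to its holster on start or primary-hand drop.
; Hand-box overlaps assign primary and secondary grips; the primary attaches the gun, and Tick aims VisualRoot between both controllers when dual wielding.
; A secondary input cycles firing modes, with Double Action firing on press and release and True Semi on press only.
; Top-load reloading snaps the clip to the loader and refills ammo.
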(event Custom|ReloadWeapon
  (params (ClipRef :type Ammo%20Clip%20Base%20BP%20Object%20Reference))
  (bind _topsnaptransform (Variables|Default|GetTopSnapTransform))
  (switch Utilities|FlowControl|Switch|SwitchonReloadType (Variables|Default|GetReloadType)
    (:NewEnumerator0
      (Transformation|AttachComponentToComponent ClipRef (Variables|Default|GetLoader) "None" "KeepWorld" "KeepWorld" "KeepWorld" true)
      (Transformation|SetActorRelativeLocation ClipRef (.location _topsnaptransform))
      (Transformation|SetActorRelativeRotation ClipRef (.rotation _topsnaptransform))
      (Variables|Default|SetCurrentAmmo (Variables|Default|GetMaxAmmo)))))

(event EventBeginPlay
  ;[0.000968 1 0] Begin Play
  (Variables|Default|SetCurrentAmmo (Variables|Default|GetMaxAmmo))
  (Utilities|FlowControl|Delay 0.1)
  (CallFunction|ResettoHolster))

(event EventTick
  (params (DeltaSeconds :type Float%20%28single-precision%29))
  (bind _returnvalue (Transformation|GetActorTransform))
  ;[0.03801 0.2604 0.03803] Event Tick
  (if (and (Variables|Default|GetGrabbed?) (Variables|Default|GetDualWielding?))
    (Transformation|SetRelativeRotation (Variables|Default|GetVisualRoot) (Math|Rotator|FindLookatRotation (Math|Transform|InverseTransformLocation _returnvalue (Transformation|GetWorldLocation (Variables|/Game/VirtualRealityBP/Blueprints/BP_MotionController.BP_MotionController_C|GetMotionController (Variables|Default|GetPrimaryHand)))) (Math|Transform|InverseTransformLocation _returnvalue (Transformation|GetWorldLocation (Variables|/Game/VirtualRealityBP/Blueprints/BP_MotionController.BP_MotionController_C|GetMotionController (Variables|Default|GetSecondaryHand))))) false false)))

(event EventTriggerPressed
  ;[1 1 1] Input Events
  (switch Utilities|FlowControl|Switch|SwitchonFiringMode (Variables|Default|GetFiringMode)
    (:NewEnumerator0
      (CallFunction|FireProjectile))
    (:NewEnumerator1
      (CallFunction|FireProjectile))))

(event EventPickup
  (params (AttachTo :type Scene%20Component%20Object%20Reference))
  (Utilities|FlowControl|Sequence
    (:then_0
      (|GunPickupLogic AttachTo))
    (:then_1
      (Variables|Default|SetDualWielding? (and (Utilities|IsValid (Variables|Default|GetPrimaryHand)) (Utilities|IsValid (Variables|Default|GetSecondaryHand)))))))

(event EventDrop
  (params (Drop%20From :type BP%20Motion%20Controller%20Object%20Reference))
  (Variables|Default|SetDualWielding? false)
  (if (== Drop%20From (Variables|Default|GetPrimaryHand))
    (Variables|Default|SetGrabbed? false)
    (Variables|Default|SetPrimaryHand 0)
    (CallFunction|ResettoHolster)
    (else
      (Variables|Default|SetSecondaryHand 0))))

(event EventTriggerReleased
  ;[1 1 1] Input Events
  (switch Utilities|FlowControl|Switch|SwitchonFiringMode (Variables|Default|GetFiringMode)
    (:NewEnumerator0
      (CallFunction|FireProjectile))))

(event EventSecondaryFBPressed
  ;[1 1 1] Input Events
  (if (Utilities|Enum|Equal(Enum) (Variables|Default|GetFiringMode) "NewEnumerator2")
    (bind _output_get (Variables|Default|SetFiringMode "NewEnumerator0"))
    (Development|PrintString (Utilities|String|EnumtoString _output_get))
    (else
      (bind _result (Math|Integer|IncrementInt (Math|Conversions|ToInteger(Byte) (Variables|Default|GetFiringMode)))
        (:%20%20
          (bind _output_get_2 (Variables|Default|SetFiringMode (Utilities|Enum|ByteToEnumFiringMode (Math|Conversions|ToByte(Integer) _result))))
          (Development|PrintString (Utilities|String|EnumtoString _output_get_2)))))))

(fn ConstructionScript)

(fn FireProjectile
  (bind _projectilearrow (Variables|Default|GetProjectileArrow))
  (bind _returnvalue (Transformation|GetWorldTransform _projectilearrow))
  (if (> (Variables|Default|GetCurrentAmmo) 0)
    (Math|Integer|DecrementInt (Variables|Default|GetCurrentAmmo)
      (:%20%20
        (Game|SpawnActorfromClass "/Game/Blueprints/Paintball_Projectile_BP.Paintball_Projectile_BP_C" (Math|Transform|MakeTransform (.location _returnvalue) (.rotation _returnvalue) "1,1,1") "Undefined" 0 (CallFunction|GetPlayerEmissiveColor) self (Variables|Default|GetFPS) 0)
        (Components|Activation|Activate (Variables|Default|GetProjectileSFX) true)))
    (else
      (Audio|PlaySound2D "/Engine/VREditor/Sounds/UI/Camera_Shutter.Camera_Shutter" 1.0 1.0 0.0 0 0))))

(fn DecipherPrimarySecondary
  (params (MotionController :type Scene%20Component%20Object%20Reference))
  (if (!= (Utilities|Array|FindItem (Class|PrimitiveComponent|GetOverlappingComponents (Variables|Default|GetPrimaryHandBox)) (.AsPrimitive%20Component (Utilities|Casting|CastToPrimitiveComponent MotionController))) -1)
    (Variables|Default|SetPrimaryHand (.AsBP%20Motion%20Controller (Utilities|Casting|CastToBP_MotionController (Components|GetOwner MotionController))))
    (elif (!= (Utilities|Array|FindItem (Class|PrimitiveComponent|GetOverlappingComponents (Variables|Default|GetSecondaryHandBox)) (.AsPrimitive%20Component (Utilities|Casting|CastToPrimitiveComponent MotionController))) -1)
      (Variables|Default|SetSecondaryHand (.AsBP%20Motion%20Controller (Utilities|Casting|CastToBP_MotionController (Components|GetOwner MotionController)))))))

(fn ResettoHolster
  (bind _holsterref (Variables|Default|GetHolsterRef))
  (Utilities|IsValid _holsterref
    (:Is%20Valid
      (Transformation|AttachComponentToComponent (Variables|/Game/Blueprints/GunHolster_BP.GunHolster_BP_C|GetGunAnchor _holsterref) "None" "SnapToTarget" "KeepWorld" "KeepWorld" true)
      (Transformation|SetRelativeRotation (Variables|Default|GetVisualRoot) "0, 0, 0" false false)
      (Transformation|SetRelativeRotation (Variables|Default|GetDefaultSceneRoot) "0, 0, 0" false false))))