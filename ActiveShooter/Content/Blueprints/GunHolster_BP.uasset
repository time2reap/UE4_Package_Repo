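; Gun holster actor that follows the player's camera, sitting below it and to the right, roughly at hip position.
; Each Tick it moves to the camera location plus small forward, larger right and fixed world-down offsets, without sweeping.
; Its rotation takes only the camera's yaw, so it stays upright when the view tilts.
; Tick fetches the player reference whenever it is invalid.
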(event EventBeginPlay)

(event EventTick
  (params (DeltaSeconds :type Float%20%28single-precision%29))
  (Utilities|IsValid (Variables|Default|GetPlayerRef)
    (:Is%20Valid
      (Transformation|SetActorLocation (+ (Transformation|GetWorldLocation (Variables|/Game/VirtualRealityBP/Blueprints/MotionControllerPawn.MotionControllerPawn_C|GetCamera (Variables|Default|GetPlayerRef))) (* (Math|Vector|GetForwardVector (Variables|/Game/VirtualRealityBP/Blueprints/MotionControllerPawn.MotionControllerPawn_C|GetCamera (Variables|Default|GetPlayerRef))) 5.0) (* (Math|Vector|GetRightVector (Variables|/Game/VirtualRealityBP/Blueprints/MotionControllerPawn.MotionControllerPawn_C|GetCamera (Variables|Default|GetPlayerRef))) 25.0) (Math|Vector|MakeVector 0.0 0.0 -5e+01)) false false)
      (Transformation|SetActorRotation (Math|Rotator|MakeRotator 0.0 0.0 (.yaw (Transformation|GetWorldRotation (Variables|/Game/VirtualRealityBP/Blueprints/MotionControllerPawn.MotionControllerPawn_C|GetCamera (Variables|Default|GetPlayerRef)))))))
    (:Is%20Not%20Valid
      (Variables|Default|SetPlayerRef (CallFunction|GetPlayerReference)))))

(fn ConstructionScript)