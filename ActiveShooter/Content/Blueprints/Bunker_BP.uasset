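; Bunker actor that takes the shape of a selectable obstacle type, with paintball-style names such as Dorito, Snake, Temple and Can.
; The construction script calls ChangeBunkerType, which maps the BunkerType variable to a basic shape mesh and a preset relative transform.
; It then applies that transform and the shared bunker material to the mesh component.
; The event graph holds no active logic.
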(event EventBeginPlay)

(event Collision|EventActorBeginOverlap
  (params (OtherActor :type Actor%20Object%20Reference)))

(event EventTick
  (params (DeltaSeconds :type Float%20%28single-precision%29)))

(fn ConstructionScript
  (CallFunction|ChangeBunkerType (Variables|Default|GetBunkerType)))

(fn ChangeBunkerType
  (params (NewType :type BunkerType%20Enum :default "NewEnumerator0"))
  (Variables|Default|SetBunkerType NewType)
  (Utilities|FlowControl|Sequence
    (:then_0
      (switch Utilities|FlowControl|Switch|SwitchonBunkerType (Variables|Default|GetBunkerType)
        (:NewEnumerator0
          (Components|StaticMesh|SetStaticMesh (Variables|Default|GetBunkerMesh) "/Game/Geometry/Meshes/1M_Cube_Chamfer.1M_Cube_Chamfer")
          (Variables|Default|SetBunkerTransform (Math|Transform|MakeTransform "0, 0,50.000000" "0, 0, 0" "1,1,1")))
        (:NewEnumerator1
          (Components|StaticMesh|SetStaticMesh (Variables|Default|GetBunkerMesh) "/Game/Geometry/Meshes/1M_Cube_Chamfer.1M_Cube_Chamfer")
          (Variables|Default|SetBunkerTransform (Math|Transform|MakeTransform "0, 0,100.000000" "0, 0, 0" "1,1,2.000000")))
        (:NewEnumerator2
          (Components|StaticMesh|SetStaticMesh (Variables|Default|GetBunkerMesh) "/Game/MobileStarterContent/Shapes/Shape_QuadPyramid.Shape_QuadPyramid")
          (Variables|Default|SetBunkerTransform (Math|Transform|MakeTransform "0, 0, 0" "0, 0, 0" "1.600000,1.600000,2.500000")))
        (:NewEnumerator3
          (Components|StaticMesh|SetStaticMesh (Variables|Default|GetBunkerMesh) "/Game/MobileStarterContent/Shapes/Shape_WideCapsule.Shape_WideCapsule")
          (Variables|Default|SetBunkerTransform (Math|Transform|MakeTransform "0, 0, 0" "0, 0, 0" "1.200000,1.200000,2.000000")))
        (:NewEnumerator4
          (Components|StaticMesh|SetStaticMesh (Variables|Default|GetBunkerMesh) "/Game/MobileStarterContent/Shapes/Shape_Pipe.Shape_Pipe")
          (Variables|Default|SetBunkerTransform (Math|Transform|MakeTransform "0, 0, 0" "0.000000,-45.000000,0.000000" "2.000000,2.000000,2.000000")))
        (:NewEnumerator5
          (Components|StaticMesh|SetStaticMesh (Variables|Default|GetBunkerMesh) "/Game/MobileStarterContent/Shapes/Shape_Pipe.Shape_Pipe")
          (Variables|Default|SetBunkerTransform (Math|Transform|MakeTransform "0, 0, 0" "0.000000,45.000000,0.000000" "2.000000,2.000000,2.000000")))
        (:NewEnumerator6
          (Components|StaticMesh|SetStaticMesh (Variables|Default|GetBunkerMesh) "/Game/MobileStarterContent/Shapes/Shape_WideCapsule.Shape_WideCapsule")
          (Variables|Default|SetBunkerTransform (Math|Transform|MakeTransform "0, 0, 0" "0, 0, 0" "0.850000,0.850000,1.400000")))
        (:NewEnumerator7
          (Components|StaticMesh|SetStaticMesh (Variables|Default|GetBunkerMesh) "/Game/MobileStarterContent/Shapes/Shape_TriPyramid.Shape_TriPyramid")
          (Variables|Default|SetBunkerTransform (Math|Transform|MakeTransform "0, 0, 0" "0,-30.000000, 0" "1.400000,1.400000,1.400000")))))
    (:then_1
      (Transformation|SetRelativeTransform (Variables|Default|GetBunkerMesh) (Variables|Default|GetBunkerTransform) false false)
      (Rendering|Material|SetMaterial (Variables|Default|GetBunkerMesh) 0 "/Game/Materials/M_Bunker.M_Bunker")
      (Rendering|Material|SetMaterial (Variables|Default|GetBunkerMesh) 1 "/Game/Materials/M_Bunker.M_Bunker"))))