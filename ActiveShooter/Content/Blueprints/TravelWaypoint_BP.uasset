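; TravelWaypoint is a selectable waypoint marker that dashes the player to its location.
; A looping or one-shot timeline bobs its arrow from BeginPlay, while highlight events toggle a box and enable/disable functions switch visuals and pointer collision.
; Select, gated by a DoOnce until ResetDash, hides the waypoint, marks it occupied, and lerps the player there via timeline-driven teleports between orange camera fades.
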(event Custom|ResetDash
  (bind _playerref (Variables|Default|GetPlayerRef))
  (Utilities|FlowControl|DoOnce false) ; enters at Reset
)

(event EventBeginPlay
  (Utilities|FlowControl|Sequence
    (:then_0
      (Variables|Default|SetPlayerRef (CallFunction|GetPlayerReference)))
    (:then_1
      (bind _alpha (Timeline|Bob_TL PlayFromStart)
        (:Update
          (Transformation|SetRelativeLocation (Variables|Default|GetArrow) (Math|Vector|Lerp(Vector) (Variables|Default|GetBotLoc) (Variables|Default|GetTopLoc) _alpha) false false))))))

(event EventSelect
  (bind _playerref (Variables|Default|GetPlayerRef))
  (Utilities|FlowControl|DoOnce false
    (:Completed
      (CallFunction|DisableWaypoint)
      (Default|CameraFadetoColor (Variables|Default|GetPlayerRef) "(R=1.000000,G=1.000000,B=1.000000,A=1.000000)" "(R=1.000000,G=0.371560,B=0.000000,A=0.700000)" 1.0)
      (Variables|Default|SetOccupied? true)
      (Variables|Default|SetPlayerStartLoc (Transformation|GetActorLocation (Variables|Default|GetPlayerRef)))
      (bind _alpha (Timeline|Dash_TL PlayFromStart)
        (:Update
          (Transformation|Teleport _playerref (Math|Vector|Lerp(Vector) (Variables|Default|GetPlayerStartLoc) (Transformation|GetActorLocation) _alpha) (Transformation|GetActorRotation _playerref)))
        (:Finished
          (Default|CameraFadetoColor (Variables|Default|GetPlayerRef) "(R=1.000000,G=0.372549,B=0.000000,A=0.701961)" "(R=1.000000,G=1.000000,B=1.000000,A=1.000000)" 1.0))))))

(event EventHighlight
  (Rendering|SetVisibility (Variables|Default|GetHighlightBox) true false))

(event EventUnhighlight
  (Rendering|SetVisibility (Variables|Default|GetHighlightBox) false false))

(fn ConstructionScript)

(fn DisableWaypoint
  (Rendering|SetVisibility (Variables|Default|GetHighlightBox) false true)
  (Collision|SetCollisionEnabled (Variables|Default|GetPointerBox) "NoCollision"))

(fn EnableWaypoint
  (Rendering|SetVisibility (Variables|Default|GetHighlightBox) true true)
  (Collision|SetCollisionEnabled (Variables|Default|GetPointerBox) "QueryOnly"))