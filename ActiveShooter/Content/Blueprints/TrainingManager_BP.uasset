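; TrainingManager_BP runs a target practice area, popping up random practice targets, tracking kills and cycling a bunker's type.
; On BeginPlay it binds to the player's debug button, gathers all PracticeTarget_BP actors and starts a self-repeating activation with random delays.
; Each round re-rolls until it finds an idle target, with no exit if none is free.
; Separate events update the kill-count text and step the bunker enum with wraparound.
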(event Custom|IncrementKillCount
  (bind _result (Math|Integer|IncrementInt (Variables|Default|GetKills))
    (:%20%20
      (Rendering|Components|TextRender|SetText (Variables|/Script/Engine.TextRenderActor|GetTextRender (Variables|Default|GetTextActor)) (Utilities|Text|ToText(String) (Utilities|String|Append "Kill Count: " (Utilities|String|ToString(Integer) _result)))))))

(event Custom|ActivateRandomTarget
  (bind _targets (Variables|Default|GetTargets))
  (Variables|Default|SetFindingTarget true)
  (while (Variables|Default|GetFindingTarget)
    (bind _output_get (Variables|Default|SetCurrentTarget (Utilities|Array|Get(acopy) _targets (Math|Random|RandomInteger (Utilities|Array|Length _targets)))))
    (if (and (not (Variables|/Game/Blueprints/PracticeTarget_BP.PracticeTarget_BP_C|GetActive? _output_get)) (not (Variables|/Game/Blueprints/PracticeTarget_BP.PracticeTarget_BP_C|GetDeactivating? _output_get)))
      (Default|Activate _output_get)
      (Variables|Default|SetFindingTarget false)))
  (Utilities|FlowControl|Delay (Math|Random|RandomFloatinRange 1.75 (Variables|Default|GetNewTargetTime)))
  (CallFunction|ActivateRandomTarget))

(event Custom|CycleBunkerType
  (bind _cyclebunker (Variables|Default|GetCycleBunker))
  (bind _bunkertype (Variables|/Game/Blueprints/Bunker_BP.Bunker_BP_C|GetBunkerType _cyclebunker))
  (if (Utilities|Enum|Equal(Enum) _bunkertype "NewEnumerator7")
    (Default|ChangeBunkerType _cyclebunker "NewEnumerator0")
    (else
      (bind _result (Math|Integer|IncrementInt (Math|Conversions|ToInteger(Byte) _bunkertype))
        (:%20%20
          (Default|ChangeBunkerType _cyclebunker (Utilities|Enum|ByteToEnumBunkerType (Math|Conversions|ToByte(Integer) _result))))))))

(event EventBeginPlay
  (bind _playerref (CallFunction|GetPlayerReference))
  (Utilities|IsValid _playerref
    (:Is%20Valid
      (bind _output_get (Variables|Default|SetPlayerRef _playerref))
      (EventDispatchers|BindEventtoDebugButtonPressed _output_get (EventDispatchers|CreateEvent :!event Custom|CycleBunkerType)))
    (:Is%20Not%20Valid
      _))
  (bind _outactors (Actor|GetAllActorsOfClass "/Game/Blueprints/PracticeTarget_BP.PracticeTarget_BP_C"))
  (Variables|Default|SetTargets _outactors)
  (CallFunction|ActivateRandomTarget))

(fn ConstructionScript)