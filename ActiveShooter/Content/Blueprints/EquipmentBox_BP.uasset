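; Equipment box that rides with the player and dispenses ammo clips for the gun when picked up from.
; Each tick it sits behind and below the player's camera, copying only its yaw, and fetches the player reference if it is invalid.
; Pickup checks GunRef's reload type and, for Top Load only, spawns a top-load clip at the AttachTo component and forwards the pickup to it.
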(event EventBeginPlay)

(event EventPickup
  (params (AttachTo :type Scene%20Component%20Object%20Reference))
  (switch Utilities|FlowControl|Switch|SwitchonReloadType (Variables|/Game/Blueprints/SciFi_Gun_BP.SciFi_Gun_BP_C|GetReloadType (Variables|Default|GetGunRef))
    (:NewEnumerator0
      (bind _returnvalue (Game|SpawnActorfromClass "/Game/Blueprints/AmmoClip_TopLoad_BP_Child.AmmoClip_TopLoad_BP_Child_C" (Math|Transform|MakeTransform (Transformation|GetWorldLocation AttachTo) "0, 0, 0" "1,1,1.000000") "Undefined" 0 0))
      (Default|Pickup _returnvalue AttachTo))))

(event EventTick
  (params (DeltaSeconds :type Float%20%28single-precision%29))
  (Utilities|IsValid (Variables|Default|GetPlayerRef)
    (:Is%20Valid
      (Transformation|SetActorLocation (+ (Transformation|GetWorldLocation (Variables|/Game/VirtualRealityBP/Blueprints/MotionControllerPawn.MotionControllerPawn_C|GetCamera (Variables|Default|GetPlayerRef))) (* (Math|Vector|GetForwardVector (Variables|/Game/VirtualRealityBP/Blueprints/MotionControllerPawn.MotionControllerPawn_C|GetCamera (Variables|Default|GetPlayerRef))) -35.0) (Math|Vector|MakeVector 0.0 0.0 -5e+01)) false false)
      (Transformation|SetActorRotation (Math|Rotator|MakeRotator 0.0 0.0 (.yaw (Transformation|GetWorldRotation (Variables|/Game/VirtualRealityBP/Blueprints/MotionControllerPawn.MotionControllerPawn_C|GetCamera (Variables|Default|GetPlayerRef)))))))
    (:Is%20Not%20Valid
      (Variables|Default|SetPlayerRef (CallFunction|GetPlayerReference)))))

(fn ConstructionScript)