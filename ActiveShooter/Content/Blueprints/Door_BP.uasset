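; VR door that a player swings by grabbing its handle with a motion controller.
; Pickup stores the hand if its GrabSphere overlaps the HandleCollider, and Drop releases it.
; While grabbed, Tick turns the root's yaw toward the controller, clamped to a fixed world-space half circle.
; Logic for deriving yaw limits from the door's own rotation is present but never runs.
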(event EventBeginPlay)

(event EventTick
  (params (DeltaSeconds :type Float%20%28single-precision%29))
  (bind _returnvalue (Transformation|GetActorLocation))
  (bind _parenthand (Variables|Default|GetParentHand))
  (bind _root (Variables|Default|GetRoot))
  (bind _returnvalue_2 (Transformation|GetWorldRotation _root))
  (bind _motioncontroller (Variables|/Game/VirtualRealityBP/Blueprints/BP_MotionController.BP_MotionController_C|GetMotionController _parenthand))
  (bind _returnvalue_3 (Transformation|GetWorldLocation _motioncontroller))
  (bind _returnvalue_4 (Math|Rotator|FindLookatRotation _returnvalue _returnvalue_3))
  (if (Variables|Default|GetGrabbed?)
    (if (> (.yaw _returnvalue_4) 0.0)
      (Variables|Default|SetNewZ (Math|Float|Clamp(Float) (.yaw _returnvalue_4) 9e+01 1.8e+02))
      (else
        (Variables|Default|SetNewZ (Math|Float|Clamp(Float) (.yaw _returnvalue_4) -1.8e+02 -9e+01))))
    (Transformation|SetWorldRotation (Variables|Default|GetRoot) (Math|Rotator|MakeRotator (.roll _returnvalue_2) (.pitch _returnvalue_2) (Variables|Default|GetNewZ)) false false)))

(event EventPickup
  (params (AttachTo :type Scene%20Component%20Object%20Reference))
  (bind _returnvalue (Components|GetOwner AttachTo))
  (bind _asbp_motion_controller (Utilities|Casting|CastToBP_MotionController _returnvalue))
  (Development|PrintString "GRABBED")
  (if (!= (Utilities|Array|FindItem (Class|PrimitiveComponent|GetOverlappingComponents (Variables|Default|GetHandleCollider)) (Variables|/Game/VirtualRealityBP/Blueprints/BP_MotionController.BP_MotionController_C|GetGrabSphere _asbp_motion_controller)) -1)
    (Variables|Default|SetGrabbed? true)
    (Variables|Default|SetParentHand _asbp_motion_controller)))

(event EventDrop
  (Variables|Default|SetGrabbed? false)
  (Variables|Default|SetParentHand 0)
  (Development|PrintString "DROPPED"))

(fn ConstructionScript)