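; Swinging paintball practice target that stays up for a limited time after activation.
; A timeline lerps the target's rotation and reverses on timeout or a hit, switching the point light's intensity when each swing finishes.
; Paintball hits pass a DoOnce, re-armed on each activation, to play a sound and, if active, trigger particles and increment the TrainingManager_BP kill count.
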(event Custom|Deactivate
  (if (not (Variables|Default|GetDeactivating?))
    (Variables|Default|SetDeactivating? true)
    (Variables|Default|SetActive? false)
    (bind _alpha (Timeline|SwingTL Reverse)
      (:Update
        (Transformation|SetRelativeRotation (Variables|Default|GetTargetRoot) (Math|Rotator|Lerp(Rotator) (Variables|Default|GetRotDe) (Variables|Default|GetRotActive) _alpha true) false false))
      (:Finished
        (if (Variables|Default|GetDeactivating?)
          (Variables|Default|SetDeactivating? false)
          (Rendering|Components|Light|SetIntensity (Variables|Default|GetPointLight) 5e+03)
          (else
            (Rendering|Components|Light|SetIntensity (Variables|Default|GetPointLight) 0.0)))))))

(event Custom|Activate
  (CallFunction|ResetTarget)
  (Variables|Default|SetActive? true)
  (Variables|Default|SetTimeLeft (Variables|Default|GetTimeToWait))
  (bind _alpha (Timeline|SwingTL PlayFromStart)
    (:Update
      (Transformation|SetRelativeRotation (Variables|Default|GetTargetRoot) (Math|Rotator|Lerp(Rotator) (Variables|Default|GetRotDe) (Variables|Default|GetRotActive) _alpha true) false false))
    (:Finished
      (if (Variables|Default|GetDeactivating?)
        (Variables|Default|SetDeactivating? false)
        (Rendering|Components|Light|SetIntensity (Variables|Default|GetPointLight) 5e+03)
        (else
          (Rendering|Components|Light|SetIntensity (Variables|Default|GetPointLight) 0.0))))))

(event Custom|ResetTarget
  (Utilities|FlowControl|DoOnce false) ; enters at Reset
)

(event EventBeginPlay
  (bind _outactors (Actor|GetAllActorsOfClass "/Game/Blueprints/TrainingManager_BP.TrainingManager_BP_C"))
  (Variables|Default|SetManager (Utilities|Array|Get(acopy) _outactors)))

(event EventShotEvent
  (params (Projectile :type Actor%20Object%20Reference) (Sender :type Actor%20Object%20Reference))
  (Utilities|Casting|CastToPaintball_Projectile_BP Projectile)
  (Utilities|FlowControl|DoOnce false
    (:Completed
      (Audio|PlaySound2D "/Game/Audio/PaintballMetalDinkHit_Cue.PaintballMetalDinkHit_Cue" 1.0 1.0 0.0 0 0)
      (if (Variables|Default|GetActive?)
        (CallFunction|Deactivate)
        (Default|IncrementKillCount (Variables|Default|GetManager))
        (Components|Activation|Activate (Variables|Default|GetHitParticle) true)))))

(event EventTick
  (params (DeltaSeconds :type Float%20%28single-precision%29))
  (if (Variables|Default|GetActive?)
    (bind _output_get (Variables|Default|SetTimeLeft (- (Variables|Default|GetTimeLeft) DeltaSeconds)))
    (if (< _output_get 0.0)
      (CallFunction|Deactivate))))

(fn ConstructionScript)