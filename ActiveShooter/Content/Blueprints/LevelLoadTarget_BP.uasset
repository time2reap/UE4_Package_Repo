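; LevelLoadTarget_BP is a shootable target that loads another level when hit by a paintball projectile.
; On a shot while active, it plays a click sound, fires its hit particle, deactivates itself and fades out the player.
; After a short delay it opens the level named in LevelToLoad.
; At BeginPlay it also caches the first TrainingManager_BP, though the shot logic does not use it.
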(event EventBeginPlay
  (bind _outactors (Actor|GetAllActorsOfClass "/Game/Blueprints/TrainingManager_BP.TrainingManager_BP_C"))
  (Variables|Default|SetManager (Utilities|Array|Get(acopy) _outactors)))

(event EventShotEvent
  (params (Projectile :type Actor%20Object%20Reference) (Sender :type Actor%20Object%20Reference))
  (if (Variables|Default|GetActive?)
    (Utilities|Casting|CastToPaintball_Projectile_BP Projectile)
    (Audio|PlaySound2D "/Engine/VREditor/Sounds/UI/Click_on_Button_Cue.Click_on_Button_Cue" 1.0 1.0 0.0 0 0)
    (Components|Activation|Activate (Variables|Default|GetHitParticle) true)
    (Variables|Default|SetActive? false)
    (Default|FadeOut (CallFunction|GetPlayerReference))
    (Utilities|FlowControl|Delay 0.5)
    (Game|OpenLevel(byName) (Utilities|String|StringToName (Variables|Default|GetLevelToLoad)))))

(fn ConstructionScript)