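; Paintball projectile that tints its mesh, impact particle and point light with the player's emissive color and takes its launch speed from LaunchSpeed.
; A hit or overlap with anything but the owning weapon feeds one shared DoOnce, so impact resolves once.
; Impact notifies Damage_Interface targets with the player as sender, stops physics and collision, plays particle and sound, removes the visual and expires shortly after.
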(event OnComponentHit(SphereCollider)
  (params (HitComponent :type Primitive%20Component%20Object%20Reference) (OtherActor :type Actor%20Object%20Reference) (OtherComp :type Primitive%20Component%20Object%20Reference) (NormalImpulse :type Vector :default "0, 0, 0") (Hit :type Hit%20Result%20Structure%20%28by%20ref%29))
  (bind _spherecollider (Variables|Default|GetSphereCollider))
  (if (!= OtherActor (Variables|Default|GetOwningWeapon))
    (Utilities|FlowControl|DoOnce false
      (:Completed
        (if (Utilities|DoesObjectImplementInterface OtherActor "/Game/Interface/Damage_Interface.Damage_Interface_C")
          (Class|DamageInterface|ShotEvent(Message) OtherActor self (CallFunction|GetPlayerReference)))
        (Physics|SetSimulatePhysics _spherecollider false)
        (Collision|SetCollisionEnabled _spherecollider "NoCollision")
        (Class|PrimitiveComponent|SetAllPhysicsLinearVelocity _spherecollider "0, 0, 0" false)
        (Components|Activation|Activate (Variables|Default|GetImpactParticle) true)
        (Actor|SetLifeSpan 1.0)
        (Components|DestroyComponent (Variables|Default|GetVisual))))))

(event EventBeginPlay
  (CallFunction|SetColor (CallFunction|GetPlayerEmissiveColor)))

(event Collision|EventActorBeginOverlap
  (params (OtherActor :type Actor%20Object%20Reference))
  (bind _spherecollider (Variables|Default|GetSphereCollider))
  (if (!= (Variables|Default|GetOwningWeapon) OtherActor)
    (Utilities|FlowControl|DoOnce false
      (:Completed
        (if (Utilities|DoesObjectImplementInterface (stale OnComponentHit(SphereCollider) OtherActor) "/Game/Interface/Damage_Interface.Damage_Interface_C")
          (Class|DamageInterface|ShotEvent(Message) (stale OnComponentHit(SphereCollider) OtherActor) self (CallFunction|GetPlayerReference)))
        (Physics|SetSimulatePhysics _spherecollider false)
        (Collision|SetCollisionEnabled _spherecollider "NoCollision")
        (Class|PrimitiveComponent|SetAllPhysicsLinearVelocity _spherecollider "0, 0, 0" false)
        (Components|Activation|Activate (Variables|Default|GetImpactParticle) true)
        (Actor|SetLifeSpan 1.0)
        (Components|DestroyComponent (Variables|Default|GetVisual))))))

(fn ConstructionScript
  (Variables|/Script/Engine.ProjectileMovementComponent|SetInitialSpeed (Variables|Default|GetProjectileMovement) (Variables|Default|GetLaunchSpeed)))

(fn SetColor
  (params (NewColor :type Linear%20Color%20Structure))
  (bind _returnvalue (Math|Conversions|ToVector(LinearColor) NewColor))
  (Rendering|Material|SetVectorParameterValueonMaterials (Variables|Default|GetVisual) "Color" _returnvalue)
  (Effects|Components|ParticleSystem|SetVectorParameter (Variables|Default|GetImpactParticle) "Color" _returnvalue)
  (Rendering|Components|Light|SetLightColor (Variables|Default|GetPointLight) NewColor true))