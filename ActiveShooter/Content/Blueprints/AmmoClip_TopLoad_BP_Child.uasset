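; An ammo clip Blueprint that can be picked up and loaded into a sci-fi gun.
; When its LoaderBox overlaps a component tagged "Loader" on a SciFi_Gun_BP, it marks itself Loaded and passes itself to that gun's ReloadWeapon, ignoring further overlaps while loaded.
; Pickup attaches the clip to the supplied component, then snaps its relative location and rotation to GrabTransform.
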(event OnComponentBeginOverlap(LoaderBox)
  (params (OverlappedComponent :type Primitive%20Component%20Object%20Reference) (OtherActor :type Actor%20Object%20Reference) (OtherComp :type Primitive%20Component%20Object%20Reference) (OtherBodyIndex :type Integer) (bFromSweep :type Boolean) (SweepResult :type Hit%20Result%20Structure%20%28by%20ref%29))
  (if (and (Components|ComponentHasTag OtherComp "Loader") (not (Variables|Default|GetLoaded?)))
    (bind _assci_fi_gun_bp (Utilities|Casting|CastToSciFi_Gun_BP OtherActor))
    (Variables|Default|SetLoaded? true)
    (Default|ReloadWeapon _assci_fi_gun_bp self)))

(event EventBeginPlay
  (|CallParentFunction) ; This node is disabled and will not be called.\nDrag off pins to build functionality.
)

(event Collision|EventActorBeginOverlap
  (params (OtherActor :type Actor%20Object%20Reference))
  (|CallParentFunction OtherActor) ; This node is disabled and will not be called.\nDrag off pins to build functionality.
)

(event EventTick
  (params (DeltaSeconds :type Float%20%28single-precision%29))
  (|CallParentFunction DeltaSeconds) ; This node is disabled and will not be called.\nDrag off pins to build functionality.
)

(event EventPickup
  (params (AttachTo :type Scene%20Component%20Object%20Reference))
  (bind _grabtransform (Variables|Default|GetGrabTransform))
  (Transformation|AttachComponentToComponent AttachTo "None" "KeepWorld" "KeepWorld" "KeepWorld" true)
  (Transformation|SetActorRelativeLocation (.location _grabtransform))
  (Transformation|SetActorRelativeRotation (.rotation _grabtransform)))

(fn ConstructionScript
  (|CallParentFunction))