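; VR katana sheath that rides at the player's left hip, can be grabbed by a motion controller, and receives the katana.
; When released, it follows a camera-derived anchor at an offset, yawing with the player or aiming at the sword hand while sheathing.
; When held, it drops beyond a distance from that anchor; tip overlap starts sheathing by attaching the katana.
; Two-handed orientation (DualWield) only prints a rotation; its SetWorldRotation is unwired.
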(event OnComponentBeginOverlap(SheathSocket)
  (params (OverlappedComponent :type Primitive%20Component%20Object%20Reference) (OtherActor :type Actor%20Object%20Reference) (OtherComp :type Primitive%20Component%20Object%20Reference) (OtherBodyIndex :type Integer) (bFromSweep :type Boolean) (SweepResult :type Hit%20Result%20Structure%20%28by%20ref%29))
  ;[0.1874 1 0.9901] Collision with Katana Tip
  (if (Components|ComponentHasTag OtherComp "KatanaTip")
    (if (and (Variables|Default|GetGrabbed) (not (Variables|Default|GetSheathing?)))
      (bind _askatana_bp (Utilities|Casting|CastToKatana_BP (Components|GetOwner OtherComp)))
      (if (Variables|/Game/Blueprints/Katana_BP.Katana_BP_C|GetCanSheath? _askatana_bp)
        (Variables|/Game/Blueprints/Katana_BP.Katana_BP_C|SetSheathing? _askatana_bp true)
        (Variables|/Game/Blueprints/Katana_BP.Katana_BP_C|SetCanDraw? _askatana_bp false)
        (CallFunction|StartSheathing)))))

(event Custom|StopSheathing
  ;[1 0.4843 0.1465] Stop Sheathing
  (Variables|Default|SetSheathing? false))

(event Custom|StartSheathing
  (bind _swordref (Variables|Default|GetSwordRef))
  (bind _swordref_2 (Variables|Default|GetSwordRef))
  ;[0.1419 1 0.5265] Start Sheathing
  (Utilities|IsValid (Variables|Default|GetSwordRef)
    (:Is%20Valid
      (Variables|Default|SetSheathing? true)
      (if (!= (Components|GetOwner _swordref_2) self)
        (Transformation|DetachFromActor _swordref_2 "KeepWorld" "KeepWorld" "KeepWorld")
        (Transformation|AttachComponentToComponent (Variables|Default|GetSwordRef) (Variables|Default|GetSheath) "None" "KeepWorld" "KeepWorld" "KeepWorld" true)
        (if (not (Variables|/Game/Blueprints/Katana_BP.Katana_BP_C|GetSheathed? (Variables|Default|GetSwordRef)))
          (bind _percentunsheathed_ (Default|CalculatePercentSheathed _swordref))
          (Default|MoveKatanainSheath _swordref _percentunsheathed_))))))

(event Custom|ResetGrabAttach
  ;[0 0 0] Event Tick
  (Utilities|FlowControl|DoOnce false) ; enters at Reset
)

(event EventBeginPlay
  ;[0.947 0.1521 1] Begin Play
  (bind _askatana_bp (Utilities|Casting|CastToKatana_BP (Variables|/Script/Engine.ChildActorComponent|GetChildActor (Variables|Default|GetKatanaActor))))
  (bind _output_get (Variables|Default|SetSwordRef _askatana_bp))
  (Variables|/Game/Blueprints/Katana_BP.Katana_BP_C|SetSheathRef _output_get self))

(event EventPickup
  (params (AttachTo :type Scene%20Component%20Object%20Reference))
  ;[0 1 0.07963] Event Pickup
  (bind _asbp_motion_controller (Utilities|Casting|CastToBP_MotionController (Components|GetOwner AttachTo)))
  (Variables|Default|SetHandRef _asbp_motion_controller)
  (Variables|Default|SetGrabbed true))

(event EventTick
  (params (DeltaSeconds :type Float%20%28single-precision%29))
  ;[0 0 0] Event Tick
  (if (Variables|Default|GetGrabbed)
    (if (Variables|Default|GetSheathing?)
      (CallFunction|DualWield)
      (else
        (Utilities|FlowControl|Sequence
          (:then_0
            (Utilities|FlowControl|DoOnce false
              (:Completed
                (CallFunction|AttachtoHand))))
          (:then_1
            (bind _newanchorpoint (CallFunction|FindAnchoronPlayer))
            (Variables|Default|SetAnchorPoint _newanchorpoint)
            (bind _toofar_ (CallFunction|CheckDistancetoAnchor))
            (if _toofar_
              (CallFunction|Drop))))))
    (else
      (Utilities|FlowControl|Sequence
        (:then_0
          (bind _newanchorpoint_2 (CallFunction|FindAnchoronPlayer))
          (Transformation|SetActorLocation (+ _newanchorpoint_2 (Variables|Default|GetAnchorOffset)) false false))
        (:then_1
          (if (Variables|Default|GetSheathing?)
            (CallFunction|OrienttoBlade)
            (else
              (CallFunction|OrienttoPlayer))))))))

(event EventDrop
  ;[1 0 0.04265] Event Drop
  (Variables|Default|SetGrabbed false)
  (Variables|Default|SetHandRef 0)
  (CallFunction|ResetGrabAttach)
  (if (Variables|Default|GetAttachedToHand?)
    (Transformation|DetachFromActor "KeepWorld" "KeepWorld" "KeepWorld"))
  (Variables|Default|SetAttachedToHand? false)
  (bind _newanchorpoint (CallFunction|FindAnchoronPlayer))
  (Variables|Default|SetAnchorOffset (- (Transformation|GetActorLocation) _newanchorpoint)))

(fn ConstructionScript)

(fn FindAnchoronPlayer
  (bind _player (Variables|Default|GetPlayer))
  (bind _camera (Variables|/Game/VirtualRealityBP/Blueprints/MotionControllerPawn.MotionControllerPawn_C|GetCamera _player))
  (bind _returnvalue (Math|Vector|GetRightVector _camera))
  (bind _returnvalue_2 (Transformation|GetWorldLocation _camera))
  (bind _returnvalue_3 (Math|Vector|GetForwardVector _camera))
  (bind _returnvalue_4 (* _returnvalue_3 1.0))
  (bind _returnvalue_5 (* _returnvalue -2e+01))
  (bind _returnvalue_6 (+ _returnvalue_2 _returnvalue_5))
  (bind _returnvalue_7 (+ _returnvalue_6 _returnvalue_4))
  (bind (_x _y) (Math|Vector|BreakVector _returnvalue_7))
  (Utilities|IsValid _player
    (:Is%20Valid
      (return (Math|Vector|MakeVector _x _y (- (.z (Transformation|GetWorldLocation (Variables|/Game/VirtualRealityBP/Blueprints/MotionControllerPawn.MotionControllerPawn_C|GetCamera (Variables|Default|GetPlayer)))) 45.0))))))

(fn OrienttoPlayer
  (bind _player (Variables|Default|GetPlayer))
  (bind _sheath_root (Variables|Default|GetSheath_Root))
  (bind _returnvalue (Transformation|GetWorldRotation _sheath_root))
  (bind _vrorigin (Variables|/Game/VirtualRealityBP/Blueprints/MotionControllerPawn.MotionControllerPawn_C|GetVROrigin _player))
  (bind _camera (Variables|/Game/VirtualRealityBP/Blueprints/MotionControllerPawn.MotionControllerPawn_C|GetCamera _player))
  (bind _returnvalue_2 (Transformation|GetWorldLocation _vrorigin))
  (bind _returnvalue_3 (Math|Vector|GetForwardVector _camera))
  (Utilities|IsValid _player
    (:Is%20Valid
      (Transformation|SetWorldRotation _sheath_root (Math|Rotator|MakeRotator (.roll _returnvalue) (.pitch _returnvalue) (.yaw (Math|Rotator|FindLookatRotation _returnvalue_2 (+ _returnvalue_2 (* (Math|Vector|MakeVector (.x _returnvalue_3) (.y _returnvalue_3) 1.5e+02) 1e+02))))) false false))))

(fn OrienttoBlade
  (bind _sheath_root (Variables|Default|GetSheath_Root))
  (bind _curveoffsetz (Variables|Default|GetCurveOffsetZ))
  (bind _swordref (Variables|Default|GetSwordRef))
  (bind _sheathsocket (Variables|Default|GetSheathSocket))
  (bind _returnvalue (Transformation|GetWorldLocation _sheathsocket))
  (bind _percentunsheathed (Variables|/Game/Blueprints/Katana_BP.Katana_BP_C|GetPercentUnSheathed _swordref))
  (bind _parenthand (Variables|/Game/Blueprints/Katana_BP.Katana_BP_C|GetParentHand _swordref))
  (bind _returnvalue_2 (* _percentunsheathed _curveoffsetz))
  (bind _handcenter (Variables|/Game/VirtualRealityBP/Blueprints/BP_MotionController.BP_MotionController_C|GetHandCenter _parenthand))
  (bind _returnvalue_3 (Math|Float|Clamp(Float) _returnvalue_2 -5e+01 -9.0))
  (bind _returnvalue_4 (Transformation|GetWorldLocation _handcenter))
  (bind _returnvalue_5 (Math|Vector|MakeVector 0.0 0.0 _returnvalue_3))
  (bind _returnvalue_6 (+ _returnvalue_4 _returnvalue_5))
  (bind _returnvalue_7 (Math|Rotator|FindLookatRotation _returnvalue _returnvalue_6))
  (Utilities|IsValid _swordref
    (:Is%20Valid
      (Rendering|Debug|DrawDebugPoint _returnvalue_6 5e+01 "(R=0.000000,G=0.936045,B=1.000000,A=1.000000)" 0.0)
      (Transformation|SetWorldRotation _sheath_root (Math|Rotator|MakeRotator (.roll (Transformation|GetWorldRotation _sheath_root)) (.pitch _returnvalue_7) (.yaw _returnvalue_7)) false false))))

(fn AttachtoHand
  (bind _handref (Variables|Default|GetHandRef))
  (Utilities|IsValid _handref
    (:Is%20Valid
      (Transformation|AttachComponentToComponent (Variables|/Game/VirtualRealityBP/Blueprints/BP_MotionController.BP_MotionController_C|GetMotionController _handref) "None" "KeepWorld" "KeepWorld" "KeepWorld" true)
      (Variables|Default|SetAttachedToHand? true)
      (Transformation|SetActorRelativeRotation (Variables|Default|GetRelativeRot))
      (Transformation|SetActorRelativeLocation (Variables|Default|GetRelativeLoc)))))

(fn DualWield
  (bind _swordref (Variables|Default|GetSwordRef))
  (Utilities|IsValid _swordref
    (:Is%20Valid
      (Development|PrintString (Utilities|String|ToString(Rotator) (Math|Rotator|FindLookatRotation (Math|Transform|InverseTransformLocation (Transformation|GetActorTransform) (Transformation|GetWorldLocation (Variables|/Game/VirtualRealityBP/Blueprints/BP_MotionController.BP_MotionController_C|GetHandCenter (Variables|Default|GetHandRef)))) (Math|Transform|InverseTransformLocation (Transformation|GetActorTransform) (Transformation|GetWorldLocation (Variables|/Game/VirtualRealityBP/Blueprints/BP_MotionController.BP_MotionController_C|GetHandCenter (Variables|/Game/Blueprints/Katana_BP.Katana_BP_C|GetParentHand _swordref)))))) true true "(R=0.460642,G=0.304575,B=1.000000,A=1.000000)"))))

(fn CheckDistancetoAnchor
  (return (> (CallFunction|GetDistancetoPoint (Transformation|GetWorldLocation (Variables|/Game/VirtualRealityBP/Blueprints/BP_MotionController.BP_MotionController_C|GetHandCenter (Variables|Default|GetHandRef))) (+ (Variables|Default|GetAnchorPoint) (Variables|Default|GetAnchorOffset)) false true false 0.0) (Variables|Default|GetMaxSheathDistance))))