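; VR pickup bundle of ninja stars that attaches to a motion controller, swapping world meshes for hand meshes tinted in the player's color.
; On drop, squared distance from LastFrameLocation decides between a throw and restoring the world meshes.
; A throw spawns three NinjaStar_BP actors fanned along the controller's forward vector and destroys the bundle.
; LastFrameLocation is only updated in unconnected debug code, and GetLaunchDirection is unused.
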(event Custom|ThrowShuriken
  (bind _parenthand (Variables|Default|GetParentHand))
  (bind _parenthand_2 (Variables|Default|GetParentHand))
  (bind _spawnoffsets (Variables|Default|GetSpawnOffsets))
  (bind _motioncontroller (Variables|/Game/VirtualRealityBP/Blueprints/BP_MotionController.BP_MotionController_C|GetMotionController _parenthand))
  (bind _motioncontroller_2 (Variables|/Game/VirtualRealityBP/Blueprints/BP_MotionController.BP_MotionController_C|GetMotionController _parenthand_2))
  (bind _returnvalue (Math|Vector|GetForwardVector _motioncontroller))
  (bind _returnvalue_2 (Transformation|GetWorldLocation _motioncontroller_2))
  (bind _returnvalue_3 (Math|Vector|GetRightVector _motioncontroller))
  (bind _returnvalue_4 (* _returnvalue_3 5.0))
  (bind _returnvalue_5 (* _returnvalue 25.0))
  (bind _returnvalue_6 (* _returnvalue_3 -5.0))
  (bind (_x _y _z) (Math|Vector|BreakVector _returnvalue_5))
  (bind _returnvalue_7 (+ _returnvalue_6 _returnvalue_5))
  (bind _returnvalue_8 (+ _returnvalue_4 _returnvalue_5))
  (Variables|Default|SetThrown? false)
  (Utilities|Array|SetArrayElem _spawnoffsets 0 (Math|Vector|MakeVector (.x _returnvalue_8) (.y _returnvalue_8) _z) true)
  (Utilities|Array|SetArrayElem _spawnoffsets 1 (Math|Vector|MakeVector _x _y _z) true)
  (Utilities|Array|SetArrayElem _spawnoffsets 2 (Math|Vector|MakeVector (.x _returnvalue_7) (.y _returnvalue_7) _z) true)
  (for _index (range 0 2)
    (Game|SpawnActorfromClass "/Game/Blueprints/NinjaStar_BP.NinjaStar_BP_C" (Math|Transform|MakeTransform (+ _returnvalue_2 (Utilities|Array|Get(acopy) (Variables|Default|GetSpawnOffsets) _index)) (Math|Rotator|FindLookatRotation _returnvalue_2 (+ _returnvalue_2 (Utilities|Array|Get(acopy) (Variables|Default|GetSpawnOffsets) _index)))) "Undefined" 0 (Variables|Default|GetParentHand) true 7e+02 "1.000000,0.000000,0.000000" (Variables|Default|GetPlayerColor) false 0)
    (Actor|DestroyActor)))

(event EventPickup
  (params (AttachTo :type Scene%20Component%20Object%20Reference))
  (bind _asbp_motion_controller (Utilities|Casting|CastToBP_MotionController (Components|GetOwner AttachTo)))
  (Variables|Default|SetParentHand _asbp_motion_controller)
  (Transformation|AttachComponentToComponent AttachTo "None" "KeepWorld" "KeepWorld" "KeepWorld" true)
  (Physics|SetSimulatePhysics (Variables|Default|GetBox) false)
  (CallFunction|ToggleWorldVisibility false)
  (CallFunction|ToggleHandVisibility true)
  (Transformation|SetActorRelativeLocation "0, 0, 0")
  (Transformation|SetActorRelativeRotation "0, 0, 0")
  (Variables|Default|SetThrown? false)
  (Variables|Default|SetPlayerColor (Variables|/Game/VirtualRealityBP/Blueprints/MotionControllerPawn.MotionControllerPawn_C|GetPlayerColor (Variables|/Game/VirtualRealityBP/Blueprints/BP_MotionController.BP_MotionController_C|GetPlayerPawn (Variables|Default|GetParentHand))))
  (CallFunction|SetStarColor))

(event EventDrop
  (params (DetachFrom :type Scene%20Component%20Object%20Reference))
  (Transformation|DetachFromActor "KeepWorld" "KeepWorld" "KeepWorld")
  (bind _throwvelocity (CallFunction|FindVelocity))
  (if (> _throwvelocity (Variables|Default|GetMinThrowVelocity))
    (CallFunction|ToggleHandVisibility false)
    (CallFunction|ThrowShuriken)
    (else
      (CallFunction|ToggleWorldVisibility true)
      (CallFunction|ToggleHandVisibility false)
      (Physics|SetSimulatePhysics (Variables|Default|GetBox) false))))

(fn ConstructionScript)

(fn GetLaunchDirection
  (bind _parenthand (Variables|Default|GetParentHand))
  (LocalVariables|SetDirectionVector (- (Transformation|GetWorldLocation (Variables|/Game/VirtualRealityBP/Blueprints/BP_MotionController.BP_MotionController_C|GetMotionController _parenthand)) (Transformation|GetWorldLocation (Variables|/Game/VirtualRealityBP/Blueprints/MotionControllerPawn.MotionControllerPawn_C|GetCamera (Variables|/Game/VirtualRealityBP/Blueprints/BP_MotionController.BP_MotionController_C|GetPlayerPawn _parenthand)))))
  (return (LocalVariables|GetDirectionVector)))

(fn ToggleWorldVisibility
  (params (Visible? :type Boolean))
  (Rendering|SetVisibility (Variables|Default|GetStar4) Visible? false))

(fn ToggleHandVisibility
  (params (Visible? :type Boolean))
  (Rendering|SetVisibility (Variables|Default|GetStar1) Visible? false))

(fn FindVelocity
  (return (Math|Vector|VectorLengthSquared (- (Transformation|GetActorLocation) (Variables|Default|GetLastFrameLocation)))))

(fn SetStarColor
  (bind _playercolor (Variables|Default|GetPlayerColor))
  (bind _star1 (Variables|Default|GetStar1))
  (Rendering|Material|SetVectorParameterValueonMaterials _star1 "Color" (Math|Vector|MakeVector (.r _playercolor) (.g _playercolor) (.b _playercolor)))
  (Rendering|Material|SetScalarParameterValueonMaterials _star1 "Boost" 3e+01))