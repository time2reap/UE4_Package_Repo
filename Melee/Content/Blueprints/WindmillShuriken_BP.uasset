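; VR throwable windmill shuriken that takes the player's color, slices sliceable meshes and sticks into world geometry.
; Dropping it from the motion controller above a speed threshold launches it gravity-free along controller forward, with speed-scaled force, spin and trail.
; Overlap begin caches the blade plane per procedural mesh, and overlap end cuts there, tinting and pushing the new half.
; Other static or dynamic hits attach it, ending in a timed smoke poof.
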(event OnComponentBeginOverlap(HitBox)
  (params (OverlappedComponent :type Primitive%20Component%20Object%20Reference) (OtherActor :type Actor%20Object%20Reference) (OtherComp :type Primitive%20Component%20Object%20Reference) (OtherBodyIndex :type Integer) (bFromSweep :type Boolean) (SweepResult :type Hit%20Result%20Structure%20%28by%20ref%29))
  (bind _returnvalue (Collision|GetCollisionObjectType OtherComp))
  (bind _proceduralplane (Variables|Default|GetProceduralPlane))
  ;[0.9091 0.2668 1] Overlap Events
  (if (Variables|Default|GetThrown?)
    (bind _assliceable_mesh_bp (Utilities|Casting|CastToSliceableMesh_BP OtherActor)
      (:then
        (Utilities|Map|Add (Variables|Default|GetSliceMap) (Variables|/Game/Blueprints/SliceableMesh_BP.SliceableMesh_BP_C|GetProceduralMeshVisual _assliceable_mesh_bp) (Utilities|Struct|MakeSliceInfo (Transformation|GetWorldLocation _proceduralplane) (Math|Vector|GetUpVector _proceduralplane))))
      (:CastFailed
        (if (or (Utilities|Enum|Equal(Enum) _returnvalue "ECC_WorldStatic") (Utilities|Enum|Equal(Enum) _returnvalue "ECC_WorldDynamic"))
          (Variables|Default|SetCanCut? false)
          (Variables|Default|SetThrown? false)
          (Utilities|FlowControl|Sequence
            (:then_0
              (CallFunction|AttachShurikentoActor OtherComp))
            (:then_1
              (Utilities|FlowControl|DoOnce false
                (:Completed
                  (Utilities|FlowControl|Delay (Variables|Default|GetTimeTilDeath))
                  (CallFunction|SmokePoof))))))))))

(event OnComponentEndOverlap(HitBox)
  (params (OverlappedComponent :type Primitive%20Component%20Object%20Reference) (OtherActor :type Actor%20Object%20Reference) (OtherComp :type Primitive%20Component%20Object%20Reference) (OtherBodyIndex :type Integer))
  ;[0.9091 0.2668 1] Overlap Events
  (if (Variables|Default|GetThrown?)
    (bind _asprocedural_mesh_component (Utilities|Casting|CastToProceduralMeshComponent OtherComp))
    (if (.ReturnValue (Utilities|Map|Find (Variables|Default|GetSliceMap) _asprocedural_mesh_component))
      (Utilities|FlowControl|Sequence
        (:then_0
          (bind _outotherhalfprocmesh (Class|KismetProceduralMeshLibrary|SliceProceduralMesh _asprocedural_mesh_component (.SlicePosition (Utilities|Struct|BreakSliceInfo (.Value (Utilities|Map|Find (Variables|Default|GetSliceMap) _asprocedural_mesh_component)))) (.SliceNormal (Utilities|Struct|BreakSliceInfo (.Value (Utilities|Map|Find (Variables|Default|GetSliceMap) _asprocedural_mesh_component)))) true "CreateNewSectionForCap" "/Game/Materials/M_GlowMat.M_GlowMat"))
          (Rendering|Material|SetVectorParameterValueonMaterials _outotherhalfprocmesh "Color" (Math|Conversions|ToVector(LinearColor) (Variables|Default|GetPlayerColor)))
          (Physics|SetSimulatePhysics _outotherhalfprocmesh true)
          (Physics|AddRadialImpulse _outotherhalfprocmesh (.SlicePosition (Utilities|Struct|BreakSliceInfo (.Value (Utilities|Map|Find (Variables|Default|GetSliceMap) _asprocedural_mesh_component)))) 3e+02 5e+02 "RIF_Constant" true)
          (Variables|/Script/Engine.ActorComponent|SetComponentTags _outotherhalfprocmesh (Utilities|Array|MakeArray "SlicedBit"))
          (Collision|SetCollisionObjectType _outotherhalfprocmesh "ECC_GameTraceChannel1"))
        (:then_1
          (Utilities|Map|Remove (Variables|Default|GetSliceMap) 0))))))

(event Custom|ThrowShuriken
  (params (ThrowDir :type Vector) (ThrowScalar :type Float%20%28single-precision%29))
  (bind _grabbox (Variables|Default|GetGrabBox))
  ;[0.1289 0.2903 1] Throw Shuriken Event
  (Utilities|FlowControl|Sequence
    (:then_0
      (Variables|Default|SetThrown? true)
      (Variables|Default|SetSpinning? true)
      (Variables|Default|SetCanCut? true)
      (Physics|SetEnableGravity _grabbox false)
      (Collision|SetCollisionEnabled _grabbox "PhysicsOnly")
      (Collision|SetCollisionEnabled (Variables|Default|GetHitBox) "QueryOnly")
      (CallFunction|CalculateRotateRate)
      (bind _output_get (Variables|Default|SetActorThrowRot (Transformation|GetWorldRotation (Variables|/Game/VirtualRealityBP/Blueprints/BP_MotionController.BP_MotionController_C|GetMotionController (Variables|Default|GetParentHand)))))
      (Transformation|SetActorRotation _output_get))
    (:then_1
      (Physics|AddForce (Variables|Default|GetGrabBox) (* ThrowDir ThrowScalar) "None" true)
      (Components|Activation|Activate (Variables|Default|GetTrailParticle) true)
      (CallFunction|ColorChangeAnim))
    (:then_2
      (Utilities|FlowControl|Delay 0.05)
      (Class|PrimitiveComponent|SetPhysicsAngularVelocityinRadians (Variables|Default|GetGrabBox) "0, 0, 0" false "None")
      (Transformation|SetWorldRotation (Variables|Default|GetVisualRoot) (Variables|Default|GetVisualThrowRot) false false)
      (Actor|SetLifeSpan (Variables|Default|GetTimeTilDeath)))))

(event Custom|ColorChangeAnim
  ;[1 1 1] Color Change Anim
  (bind _alpha (Timeline|CC_Anim PlayFromStart)
    (:Update
      (Rendering|Material|SetScalarParameterValueonMaterials (Variables|Default|GetVisual) "Boost" (Math|Float|Lerp 0.0 3e+01 _alpha)))))

(event EventBeginPlay
  ;[0 1 0.03192] Event Begin Play
  (Variables|Default|SetHalfSpinRate (Math|Random|RandomFloatinRange 3e+01 1.3e+02)))

(event EventTick
  (params (DeltaSeconds :type Float%20%28single-precision%29))
  ;[0 0 0] Event Tick
  (Utilities|FlowControl|Sequence
    (:then_0
      (Utilities|IsValid (Variables|Default|GetParentHand)
        (:Is%20Valid
          (if (not (Variables|Default|GetThrown?))
            (bind _result (Math|Integer|IncrementInt (Variables|Default|GetUpdateTicks))
              (:%20%20
                (if (> _result 5)
                  (Variables|Default|SetLastFrameLocation (Transformation|GetActorLocation))
                  (Variables|Default|SetUpdateTicks 0))))
            (elif (Variables|Default|GetSpinning?)
              (Transformation|AddLocalRotation (Variables|Default|GetVisual) (Math|Rotator|MakeRotator 0.0 0.0 (* DeltaSeconds (Variables|Default|GetRotateRate))) false false))))))
    (:then_1
      (Variables|Default|SetLastFrameLocation (Transformation|GetActorLocation)))))

(event EventPickup
  (params (AttachTo :type Scene%20Component%20Object%20Reference))
  ;[0 1 0.9705] Event Pickup
  (bind _asbp_motion_controller (Utilities|Casting|CastToBP_MotionController (Components|GetOwner AttachTo)))
  (Variables|Default|SetParentHand _asbp_motion_controller)
  (CallFunction|AttachtoParentHand AttachTo)
  (CallFunction|SetShurikenColors)
  (Components|Activation|Deactivate (Variables|Default|GetHitParticle)))

(event EventDrop
  (params (DetachFrom :type Scene%20Component%20Object%20Reference))
  ;[1 0 0.002667] Event Drop
  (Transformation|DetachFromActor "KeepWorld" "KeepWorld" "KeepWorld")
  (Variables|Default|SetVisualThrowRot (Transformation|GetWorldRotation (Variables|Default|GetVisualRoot)))
  (Physics|SetSimulatePhysics (Variables|Default|GetGrabBox) true)
  (bind _speed (CallFunction|GetSpeed))
  (if (> _speed (Variables|Default|GetMinThrowRequirement))
    (bind _direction (CallFunction|GetLaunchDirection))
    (CallFunction|ThrowShuriken _direction (Math|Float|Clamp(Float) (* (Math|Float|Clamp(Float) (/ _speed 8e+04) 0.25) (Variables|Default|GetBase%20ProjectileSpeed)) 5e+03 1e+04))))

(fn ConstructionScript)

(fn GetLaunchDirection
  (return (Math|Vector|GetForwardVector (Variables|/Game/VirtualRealityBP/Blueprints/BP_MotionController.BP_MotionController_C|GetMotionController (Variables|Default|GetParentHand)))))

(fn AttachtoParentHand
  (params (Parent :type Scene%20Component%20Object%20Reference))
  (Transformation|AttachComponentToComponent Parent "None" "KeepWorld" "KeepWorld" "KeepWorld" true)
  (Variables|Default|SetThrown? false)
  (Physics|SetSimulatePhysics (Variables|Default|GetGrabBox) false)
  (Transformation|SetActorRelativeLocation (Variables|Default|GetGrabLocation))
  (Transformation|SetActorRelativeRotation (Variables|Default|GetGrabRotation))
  (Transformation|SetRelativeLocationAndRotation (Variables|Default|GetVisual) "0, 0, 0" "0, 0, 0" false false))

(fn SetShurikenColors
  (bind _output_get (Variables|Default|SetPlayerColor (Variables|/Game/VirtualRealityBP/Blueprints/MotionControllerPawn.MotionControllerPawn_C|GetPlayerColor (Variables|/Game/VirtualRealityBP/Blueprints/BP_MotionController.BP_MotionController_C|GetPlayerPawn (Variables|Default|GetParentHand)))))
  (Rendering|Material|SetVectorParameterValueonMaterials (Variables|Default|GetVisual) "Color" (Math|Conversions|ToVector(LinearColor) _output_get))
  (Effects|Components|ParticleSystem|SetColorParameter (Variables|Default|GetHitParticle) "Start Color" _output_get)
  (Effects|Components|ParticleSystem|SetColorParameter (Variables|Default|GetDeathPoofParticle) "Color" _output_get))

(fn CalculateRotateRate
  (Variables|Default|SetHalfSpinRate (* (Variables|Default|GetHalfSpinRate) (Math|Vector|DotProduct (Transformation|GetActorUpVector) "0, 0,1.000000"))))

(fn AttachShurikentoActor
  (params (ParentComponent :type Scene%20Component%20Object%20Reference))
  (Transformation|AttachComponentToComponent ParentComponent "None" "KeepWorld" "KeepWorld" "KeepWorld" true)
  (Variables|Default|SetSpinning? false)
  (Variables|Default|SetDrifting? false)
  (Components|Activation|Deactivate (Variables|Default|GetTrailParticle))
  (Components|Activation|Activate (Variables|Default|GetHitParticle) true)
  (Actor|SetLifeSpan (Variables|Default|GetLifespanOnAttach)))

(fn SendSliceEvent
  (params (TargetObject :type Object%20Object%20Reference))
  (Class|SliceInterface|Slice(Message) TargetObject (Transformation|GetActorLocation) (Math|Vector|GetUpVector (Variables|Default|GetProceduralPlane)) (Variables|Default|GetPlayerColor)))

(fn CalculateSliceValues)

(fn SmokePoof
  (Rendering|SetVisibility (Variables|Default|GetVisual) false false)
  (Components|Activation|Activate (Variables|Default|GetDeathPoofParticle) false)
  (Actor|SetLifeSpan 1.0)
  (Audio|PlaySoundatLocation "/Game/Audio/ThrowingWeapons/SmokePoof_Cue.SmokePoof_Cue" (Transformation|GetWorldLocation (Variables|Default|GetVisual)) "0, 0, 0" 1.0 1.0 0.0 0 0 0))

(fn GetCanCut
  (return (Variables|Default|GetCanCut?)))

(fn GetCurrentVelocity
  (return (- (Transformation|GetActorLocation) (Variables|Default|GetLocLastFrame))))

(fn GetSliceColor
  (return (Variables|Default|GetPlayerColor)))

(fn GetSliceNormal
  (return (Math|Vector|GetUpVector (Variables|Default|GetProceduralPlane))))

(fn GetSpeed
  (return (/ (Math|Vector|VectorLength (- (Transformation|GetActorLocation) (Variables|Default|GetLocLastFrame))) (Utilities|Time|GetWorldDeltaSeconds))))