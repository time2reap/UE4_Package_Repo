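; Sliceable mesh actor that can be cut along a given plane into physics-simulated pieces.
; The construction script copies the chosen static mesh into a procedural mesh with collision.
; Each slice splits that mesh with a glowing cap, then colors, tags and radially launches the new half.
; Pieces are tracked up to a limit, after which slicing stops, pieces are destroyed and the actor expires shortly after.
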(event Custom|AddSlice
  (params (NewPiece :type Procedural%20Mesh%20Component%20Object%20Reference))
  (bind _meshslices (Variables|Default|GetMeshSlices))
  (if (< (Utilities|Array|Length _meshslices) (Variables|Default|GetMaxSlices))
    (Utilities|Array|AddUnique _meshslices NewPiece)
    (else
      (Variables|Default|SetSlicable? false)
      (Components|DestroyComponent NewPiece)
      (for _array_element (Variables|Default|GetMeshSlices)
        (Components|DestroyComponent _array_element))
      (Actor|SetLifeSpan 1.2))))

(event Custom|ResetSliceEvent
  (Utilities|FlowControl|DoOnce false) ; enters at Reset
)

(event EventSlice
  (params (SlicePosition :type Vector :default "0, 0, 0") (SliceNormal :type Vector :default "0, 0, 0") (SliceColor :type Linear%20Color%20Structure))
  (if (Variables|Default|GetSlicable?)
    (Utilities|FlowControl|DoOnce false
      (:Completed
        (bind _outotherhalfprocmesh (Class|KismetProceduralMeshLibrary|SliceProceduralMesh (Variables|Default|GetProceduralMeshVisual) SlicePosition SliceNormal true "CreateNewSectionForCap" "/Game/Materials/M_GlowMat.M_GlowMat"))
        (Rendering|Material|SetVectorParameterValueonMaterials _outotherhalfprocmesh "Color" (Math|Conversions|ToVector(LinearColor) SliceColor))
        (Physics|SetSimulatePhysics _outotherhalfprocmesh true)
        (CallFunction|AddSlice _outotherhalfprocmesh)
        (Physics|AddRadialImpulse _outotherhalfprocmesh SlicePosition 3e+02 5e+02 "RIF_Constant" true)
        (Variables|/Script/Engine.ActorComponent|SetComponentTags _outotherhalfprocmesh (Utilities|Array|MakeArray "SlicedBit"))
        (CallFunction|ResetSliceEvent)
        (Variables|Default|SetSliced? true)))))

(fn ConstructionScript
  (Components|StaticMesh|SetStaticMesh (Variables|Default|GetVisual) (Variables|Default|GetMesh))
  (Class|KismetProceduralMeshLibrary|CopyProceduralMeshfromStaticMeshComponent (Variables|Default|GetVisual) 0 (Variables|Default|GetProceduralMeshVisual) true))