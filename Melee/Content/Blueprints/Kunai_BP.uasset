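; VR throwable kunai that attaches to a motion controller, takes the player's color, and snaps to a forward or reverse grip.
; On release, controller speed decides between a physics drop and a gravity-free spinning throw with an oscillating trail.
; Throw direction and clamped speed come from displacement since a periodically sampled held position.
; Impacts attach it to the struck component with particles and sound, then it fades and destroys itself.
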(event OnComponentBeginOverlap(Hitbox)
  (params (OverlappedComponent :type Primitive%20Component%20Object%20Reference) (OtherActor :type Actor%20Object%20Reference) (OtherComp :type Primitive%20Component%20Object%20Reference) (OtherBodyIndex :type Integer) (bFromSweep :type Boolean) (SweepResult :type Hit%20Result%20Structure%20%28by%20ref%29))
  (bind _hitbox (Variables|Default|GetHitbox))
  ;[1 1 1] Throw Logic
  (if (Variables|Default|GetThrown?)
    (Utilities|Casting|CastToBP_MotionController OtherActor
      (:CastFailed
        (Utilities|FlowControl|DoOnce false
          (:Completed
            (Transformation|AttachComponentToComponent OtherComp "None" "KeepWorld" "KeepWorld" "KeepWorld" true)
            (Components|Activation|SetActive (Variables|Default|GetTrailEffect) false false)
            (Components|Activation|Activate (Variables|Default|GetHitParticle) true)
            (Physics|SetSimulatePhysics _hitbox false)
            (Physics|SetPhysicsLinearVelocity _hitbox "0, 0, 0" false "None")
            (Variables|Default|SetSpinning? false)
            (Audio|PlaySoundatLocation "/Game/Audio/ThrowingWeapons/ThrowingKnife_Cue.ThrowingKnife_Cue" (Transformation|GetWorldLocation (Variables|Default|GetVisualRoot)) "0, 0, 0" 1.0 1.0 0.0 0 0 0)
            (Utilities|FlowControl|Delay 4.0)
            (CallFunction|Dematerialize)))))))

(event Custom|ThrowKunai
  (bind _hitbox (Variables|Default|GetHitbox))
  ;[1 1 1] Throw Logic
  (Utilities|FlowControl|DoOnce false
    (:Completed
      (Variables|Default|SetThrown? true)
      (Physics|SetEnableGravity _hitbox false)
      (Collision|SetCollisionResponsetoAllChannels _hitbox "ECR_Overlap")
      (Variables|/Script/CableComponent.CableComponent|SetbEnableCollision (Variables|Default|GetCable) false)
      (Variables|/Script/CableComponent.CableComponent|SetbEnableCollision (Variables|Default|GetCable2) false)
      (Variables|Default|SetSpinning? true)
      (Components|Activation|Activate (Variables|Default|GetTrailEffect) true)
      (CallFunction|TrailOscilate)
      (Components|Box|SetBoxExtent (Variables|Default|GetHitbox) (Variables|Default|GetThrowExtent) true)
      (Transformation|SetRelativeLocation (Variables|Default|GetVisualRoot) (Variables|Default|GetVisualThrowLoc) false false)
      (|PhysicsThrowLogic))))

(event Custom|Dematerialize
  ;[0.1051 0.8196 1] Dematerialize
  (bind _alpha (Timeline|Timeline_0 PlayFromStart)
    (:Update
      (Rendering|Material|SetScalarParameterValueonMaterials (Variables|Default|GetBlade) "Boost" (Math|Float|Lerp 1e+02 0.0 _alpha)))
    (:Finished
      (Utilities|FlowControl|Delay 2.0)
      (Utilities|IsValid (Variables|Default|GetParentHand)
        (:Is%20Not%20Valid
          (Actor|DestroyActor))))))

(event Custom|TrailOscilate
  ;[0.8588 0.1697 1] Oscilate trail particle
  (bind _alpha (Timeline|Oscilate_TL PlayFromStart)
    (:Update
      (Transformation|SetRelativeLocation (Variables|Default|GetTrailEffect) (Math|Vector|Lerp(Vector) (Variables|Default|GetTrailLow) (Variables|Default|GetTrailHigh) _alpha) false false))))

(event Custom|ResetThrow
  (bind _hitbox (Variables|Default|GetHitbox))
  (bind _hitbox_2 (Variables|Default|GetHitbox))
  ;[1 1 1] Throw Logic
  (Utilities|FlowControl|Sequence
    (:then_0
      (Utilities|FlowControl|DoOnce false) ; enters at Reset
    )
    (:then_1
      (Utilities|FlowControl|DoOnce false) ; enters at Reset
    )
    (:then_2
      (Utilities|FlowControl|DoOnce false) ; enters at Reset
    )))

(event EventBeginPlay
  (Variables|Default|SetBoxExtent (Components|Box|GetUnscaledBoxExtent (Variables|Default|GetHitbox)))
  (Variables|Default|SetVisualLoc (Variables|/Script/Engine.SceneComponent|GetRelativeLocation (Variables|Default|GetVisualRoot))))

(event EventTick
  (params (DeltaSeconds :type Float%20%28single-precision%29))
  ;[0 0 0] Event Tick
  (if (not (Variables|Default|GetThrown?))
    (Utilities|IsValid (Variables|Default|GetParentHand)
      (:Is%20Valid
        (bind _result (Math|Integer|IncrementInt (Variables|Default|GetUpdateTicks))
          (:%20%20
            (if (> _result 1)
              (Variables|Default|SetLastFrameLocation (Transformation|GetActorLocation))
              (Variables|Default|SetUpdateTicks 0))))))
    (elif (Variables|Default|GetSpinning?)
      (Transformation|AddLocalRotation (Variables|Default|GetVisualRoot) (Math|Rotator|MakeRotator (* DeltaSeconds (Variables|Default|GetRotateRate)) 0.0 0.0) false false))))

(event EventPickup
  (params (AttachTo :type Scene%20Component%20Object%20Reference))
  ;[0.2026 1 0.2461] Event Pickup
  (bind _asbp_motion_controller (Utilities|Casting|CastToBP_MotionController (Components|GetOwner AttachTo)))
  (Variables|Default|SetParentHand _asbp_motion_controller)
  (Utilities|FlowControl|Sequence
    (:then_0
      (Transformation|AttachComponentToComponent AttachTo "None" "SnapToTarget" "KeepWorld" "KeepWorld" true)
      (CallFunction|ResetThrow)
      (Variables|Default|SetThrown? false)
      (Physics|SetSimulatePhysics (Variables|Default|GetHitbox) false)
      (Physics|SetEnableGravity (Variables|Default|GetHitbox) true)
      (Components|Activation|Deactivate (Variables|Default|GetHitParticle)))
    (:then_1
      (Components|Box|SetBoxExtent (Variables|Default|GetHitbox) (Variables|Default|GetBoxExtent) true)
      (Transformation|SetRelativeLocation (Variables|Default|GetVisualRoot) (Variables|Default|GetVisualLoc) false false)
      (bind _holdforward_ (CallFunction|GetHoldDirection))
      (if _holdforward_
        (Transformation|SetRelativeLocationAndRotation (Variables|Default|GetHitbox) (Variables|Default|GetGrabLocationForward) (Variables|Default|GetGrabRotationForward) false false)
        (CallFunction|SetKunaiColor)
        (else
          (Transformation|SetRelativeLocationAndRotation (Variables|Default|GetHitbox) (Variables|Default|GetGrabLocationBackward) (Variables|Default|GetGrabRotationBackward) false false)
          (CallFunction|SetKunaiColor))))))

(event EventDrop
  (params (DetachFrom :type Scene%20Component%20Object%20Reference))
  (bind _hitbox (Variables|Default|GetHitbox))
  ;[0.4635 0.09174 0.09174] Event Drop
  (Transformation|DetachFromActor "KeepWorld" "KeepWorld" "KeepWorld")
  (Physics|SetSimulatePhysics _hitbox true)
  (bind _speed (CallFunction|CalculateThrowSpeed))
  (if (> _speed (Variables|Default|GetMinThrowSpeed))
    (CallFunction|ThrowKunai)
    (else
      (Physics|SetEnableGravity _hitbox true)
      (Collision|SetCollisionResponsetoAllChannels _hitbox "ECR_Block"))))

(event Collision|EventHit
  (params (MyComp :type Primitive%20Component%20Object%20Reference) (Other :type Actor%20Object%20Reference) (OtherComp :type Primitive%20Component%20Object%20Reference) (bSelfMoved :type Boolean) (HitLocation :type Vector :default "0, 0, 0") (HitNormal :type Vector :default "0, 0, 0") (NormalImpulse :type Vector :default "0, 0, 0") (Hit :type Hit%20Result%20Structure%20%28by%20ref%29))
  (bind _hitbox (Variables|Default|GetHitbox))
  ;[1 1 1] Throw Logic
  (if (Variables|Default|GetThrown?)
    (Utilities|Casting|CastToBP_MotionController Other)
    (Utilities|FlowControl|DoOnce false
      (:Completed
        (Transformation|AttachComponentToComponent OtherComp "None" "KeepWorld" "KeepWorld" "KeepWorld" true)
        (Components|Activation|SetActive (Variables|Default|GetTrailEffect) false false)
        (Components|Activation|Activate (Variables|Default|GetHitParticle) true)
        (Physics|SetSimulatePhysics _hitbox false)
        (Physics|SetPhysicsLinearVelocity _hitbox "0, 0, 0" false "None")
        (Variables|Default|SetSpinning? false)
        (Audio|PlaySoundatLocation "/Game/Audio/ThrowingWeapons/ThrowingKnife_Cue.ThrowingKnife_Cue" (Transformation|GetWorldLocation (Variables|Default|GetVisualRoot)) "0, 0, 0" 1.0 1.0 0.0 0 0 0)
        (Utilities|FlowControl|Delay 4.0)
        (CallFunction|Dematerialize)))))

(fn ConstructionScript)

(fn GetLaunchDirection
  (bind _returnvalue (Transformation|GetActorLocation))
  (bind _lastframelocation (Variables|Default|GetLastFrameLocation))
  (bind _returnvalue_2 (- _returnvalue _lastframelocation))
  (LocalVariables|SetDirectionVector (Math|Vector|Normalize _returnvalue_2))
  (return (LocalVariables|GetDirectionVector) (Math|Vector|VectorLengthSquared _returnvalue_2)))

(fn SetKunaiColor
  (bind _blade (Variables|Default|GetBlade))
  (bind _parenthand (Variables|Default|GetParentHand))
  (bind _playerpawn (Variables|/Game/VirtualRealityBP/Blueprints/BP_MotionController.BP_MotionController_C|GetPlayerPawn _parenthand))
  (bind _playercolor (Variables|/Game/VirtualRealityBP/Blueprints/MotionControllerPawn.MotionControllerPawn_C|GetPlayerColor _playerpawn))
  (Rendering|Material|SetVectorParameterValueonMaterials _blade "Color" (Math|Conversions|ToVector(LinearColor) _playercolor))
  (Rendering|Material|SetScalarParameterValueonMaterials _blade "Boost" 5e+01)
  (Effects|Components|ParticleSystem|SetVectorParameter (Variables|Default|GetTrailEffect) "Start Color" (Math|Conversions|ToVector(LinearColor) _playercolor)))

(fn CalculateThrowSpeed
  (bind _parenthand (Variables|Default|GetParentHand))
  (Utilities|IsValid _parenthand
    (:Is%20Valid
      (bind _controllerspeed (Default|GetControllerSpeed _parenthand))
      (return _controllerspeed))
    (:Is%20Not%20Valid
      (return 0.0))))

(fn GetHoldDirection
  (return (> (Math|Vector|DotProduct (Math|Vector|GetRightVector (Variables|/Game/VirtualRealityBP/Blueprints/BP_MotionController.BP_MotionController_C|GetMotionController (Variables|Default|GetParentHand))) (Transformation|GetActorForwardVector)) 0.0)))