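; A VR smoke bomb that motion controllers can pick up and throw, exploding into smoke in the throwing player's color.
; Pickup attaches it to the hand, and Drop restores physics, arming it only if controller speed exceeds a throw threshold.
; Arming enables overlap queries and starts a player-colored particle effect.
; The first overlap with a static or dynamic world object hides the bomb and triggers its child Smoke_BP explosion.
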(event OnComponentBeginOverlap(BoxCollider)
  (params (OverlappedComponent :type Primitive%20Component%20Object%20Reference) (OtherActor :type Actor%20Object%20Reference) (OtherComp :type Primitive%20Component%20Object%20Reference) (OtherBodyIndex :type Integer) (bFromSweep :type Boolean) (SweepResult :type Hit%20Result%20Structure%20%28by%20ref%29))
  (bind _returnvalue (Collision|GetCollisionObjectType OtherComp))
  (bind _bomb (Variables|Default|GetBomb))
  (if (and (Variables|Default|GetAlive?) (or (Utilities|Enum|Equal(Enum) _returnvalue "ECC_WorldStatic") (Utilities|Enum|Equal(Enum) _returnvalue "ECC_WorldDynamic")))
    (Variables|Default|SetAlive? false)
    (Utilities|FlowControl|Sequence
      (:then_0
        (Components|Activation|Deactivate (Variables|Components|GetParticleSystem))
        (Rendering|SetVisibility _bomb false false)
        (Physics|SetSimulatePhysics _bomb false)
        (Collision|SetCollisionEnabled _bomb "NoCollision")
        (Physics|SetEnableGravity _bomb false))
      (:then_1
        (bind _assmoke_bp (Utilities|Casting|CastToSmoke_BP (Variables|/Script/Engine.ChildActorComponent|GetChildActor (Variables|Default|GetSmoke_BP))))
        (Default|Explode _assmoke_bp (Variables|Default|GetColor))))))

(event EventPickup
  (params (AttachTo :type Scene%20Component%20Object%20Reference))
  (if (Variables|Default|GetAlive?)
    (bind _asbp_motion_controller (Utilities|Casting|CastToBP_MotionController (Components|GetOwner AttachTo)))
    (Variables|Default|SetParentHand _asbp_motion_controller)
    (Physics|SetSimulatePhysics (Variables|Default|GetBomb) false)
    (Transformation|AttachComponentToComponent AttachTo "None" "KeepWorld" "KeepWorld" "KeepWorld" true)
    (Transformation|SetActorRelativeLocation "0, 0, 0")
    (Transformation|SetActorRelativeRotation "0, 0, 0")))

(event EventDrop
  (params (DetachFrom :type Scene%20Component%20Object%20Reference))
  (if (Variables|Default|GetAlive?)
    (bind _controllerspeed (Default|GetControllerSpeed (Variables|Default|GetParentHand)))
    (if (> _controllerspeed (Variables|Default|GetMinThrowSpeed))
      (Physics|SetSimulatePhysics (Variables|Default|GetBomb) true)
      (Transformation|DetachFromActor "KeepWorld" "KeepWorld" "KeepWorld")
      (Collision|SetCollisionEnabled (Variables|Default|GetBoxCollider) "QueryOnly")
      (CallFunction|SetSmokeColor)
      (Effects|Components|ParticleSystem|SetColorParameter (Variables|Components|GetParticleSystem) "Start Color" (Variables|Default|GetColor))
      (Components|Activation|Activate (Variables|Components|GetParticleSystem) true)
      (Variables|Default|SetParentHand 0)
      (else
        (Physics|SetSimulatePhysics (Variables|Default|GetBomb) true)
        (Transformation|DetachFromActor "KeepWorld" "KeepWorld" "KeepWorld")
        (Variables|Default|SetParentHand 0)))))

(fn ConstructionScript
  (Effects|Components|ParticleSystem|SetColorParameter (Variables|Components|GetParticleSystem) "Start Color" "(R=0.000000,G=0.970974,B=1.000000,A=1.000000)"))

(fn SetSmokeColor
  (bind _parenthand (Variables|Default|GetParentHand))
  (Utilities|IsValid _parenthand
    (:Is%20Valid
      (Variables|Default|SetColor (Variables|/Game/VirtualRealityBP/Blueprints/MotionControllerPawn.MotionControllerPawn_C|GetPlayerColor (Variables|/Game/VirtualRealityBP/Blueprints/BP_MotionController.BP_MotionController_C|GetPlayerPawn _parenthand))))))