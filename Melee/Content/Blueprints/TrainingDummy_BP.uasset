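; Training dummy Blueprint with a procedural mesh body that tracks sliced-off mesh pieces.
; The construction script copies the Visual static mesh into ProceduralMeshVisual with collision enabled.
; An AddSlice event adds a new piece uniquely to MeshSlices only when the array length exceeds MaxSlices, and otherwise destroys that piece.
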(event Custom|AddSlice
  (params (NewPiece :type Procedural%20Mesh%20Component%20Object%20Reference))
  (bind _meshslices (Variables|Default|GetMeshSlices))
  (if (> (Utilities|Array|Length _meshslices) (Variables|Default|GetMaxSlices))
    (Utilities|Array|AddUnique _meshslices NewPiece)
    (else
      (Components|DestroyComponent NewPiece))))

(event EventBeginPlay)

(event Collision|EventActorBeginOverlap
  (params (OtherActor :type Actor%20Object%20Reference)))

(event EventTick
  (params (DeltaSeconds :type Float%20%28single-precision%29)))

(fn ConstructionScript
  (Class|KismetProceduralMeshLibrary|CopyProceduralMeshfromStaticMeshComponent (Variables|Default|GetVisual) 0 (Variables|Default|GetProceduralMeshVisual) true))