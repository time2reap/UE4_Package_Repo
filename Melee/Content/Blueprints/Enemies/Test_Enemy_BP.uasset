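; Test enemy dummy for VR sword combat that can be dismembered at head, torso and limbs, then respawns through Weeb_Manager when destroyed.
; Procedural meshes copied from per-part static meshes are plane-sliced by fast "Slicer" overlaps, with the matching bone hidden and the body ragdolled.
; A low horizontal torso cut bisects it, spawning Test_Enemy_Torso_BP for the upper half.
; Cuts tint pieces with the player's color and start a five-second lifespan.
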(event OnComponentBeginOverlap(ProceduralMesh_Torso)
  (params (OverlappedComponent :type Primitive%20Component%20Object%20Reference) (OtherActor :type Actor%20Object%20Reference) (OtherComp :type Primitive%20Component%20Object%20Reference) (OtherBodyIndex :type Integer) (bFromSweep :type Boolean) (SweepResult :type Hit%20Result%20Structure%20%28by%20ref%29))
  ;[0 0.08472 1] Torso bisecct
  (if (Math|Boolean|ANDBoolean (Components|ComponentHasTag OtherComp "Slicer") (Variables|ProceduralSlicing|GetCanCutInHalf?) (not (Utilities|IsValid (Variables|Default|GetTorsoRef))))
    (bind _speed (Class|SlicerInterface|GetSpeed(Message) OtherActor))
    (if (> _speed (Variables|Default|GetMinCutSpeed))
      (Utilities|FlowControl|Sequence
        (:then_0
          (Variables|Default|SetSliceLocation (Transformation|GetWorldLocation OtherComp))
          (Variables|Default|SetSliceNormal (Math|Vector|GetUpVector OtherComp)))
        (:then_1
          (bind _canbisect_ (CallFunction|CanSliceBisect? (Variables|Default|GetSliceLocation) (Variables|Default|GetSliceNormal)))
          (if _canbisect_
            (CallFunction|SliceinHalf)
            (CallFunction|RespawnCharacter)))))))

(event OnComponentBeginOverlap(ProceduralMesh_LeftUpperLeg)
  (params (OverlappedComponent :type Primitive%20Component%20Object%20Reference) (OtherActor :type Actor%20Object%20Reference) (OtherComp :type Primitive%20Component%20Object%20Reference) (OtherBodyIndex :type Integer) (bFromSweep :type Boolean) (SweepResult :type Hit%20Result%20Structure%20%28by%20ref%29))
  (bind _proceduralmesh_lll (Variables|Default|GetProceduralMesh_LLL))
  ;[1 0.2366 0.1968] Left upper leg
  (if (and (Components|ComponentHasTag OtherComp "Slicer") (Variables|ProceduralSlicing|GetCanCutRightUpperLeg?))
    (bind _outprocmesh (CallFunction|ProceduralMeshSliceandHide OtherComp (Variables|Default|GetProceduralMesh_LeftUpperLeg) (Variables|Default|GetFallOffDir_LUL) "pelvis" "thigh_l"))
    (Utilities|IsValid _outprocmesh
      (:Is%20Valid
        (CallFunction|RespawnCharacter)
        (Variables|ProceduralSlicing|SetCanCutLeftUpperLeg? false)
        (if (Variables|ProceduralSlicing|GetCanCutLeftLowerLeg?)
          (Variables|ProceduralSlicing|SetCanCutLeftLowerLeg? false)
          (Collision|SetCollisionResponsetoAllChannels _proceduralmesh_lll "ECR_Block")
          (Collision|SetCollisionEnabled _proceduralmesh_lll "PhysicsOnly")
          (Transformation|DetachFromComponent _proceduralmesh_lll "KeepWorld" "KeepWorld" "KeepWorld" true)
          (Transformation|AttachComponentToComponent _proceduralmesh_lll _outprocmesh "None" "KeepWorld" "KeepWorld" "KeepWorld" true)
          (Rendering|SetVisibility _proceduralmesh_lll true false))))))

(event OnComponentBeginOverlap(ProceduralMesh_L_LowerArm)
  (params (OverlappedComponent :type Primitive%20Component%20Object%20Reference) (OtherActor :type Actor%20Object%20Reference) (OtherComp :type Primitive%20Component%20Object%20Reference) (OtherBodyIndex :type Integer) (bFromSweep :type Boolean) (SweepResult :type Hit%20Result%20Structure%20%28by%20ref%29))
  ;[0.04986 1 0] Left Lower Arm
  (if (Math|Boolean|ANDBoolean (Components|ComponentHasTag OtherComp "Slicer") (Variables|ProceduralSlicing|GetCanCutLeftLowerArm?) (Variables|ProceduralSlicing|GetCanCutLeftUpperArm?) (not (Utilities|IsValid (Variables|Default|GetTorsoRef))))
    (bind _outprocmesh (CallFunction|ProceduralMeshSliceandHide OtherComp (Variables|Default|GetProceduralMesh_L_LowerArm) (Variables|Default|GetFallOffDir_LLA) "upperarm_l" "lowerarm_l"))
    (Utilities|IsValid _outprocmesh
      (:Is%20Valid
        (Variables|ProceduralSlicing|SetCanCutLeftLowerArm? false)
        (CallFunction|RespawnCharacter)))))

(event OnComponentBeginOverlap(ProceduralMesh_L_UpperArm)
  (params (OverlappedComponent :type Primitive%20Component%20Object%20Reference) (OtherActor :type Actor%20Object%20Reference) (OtherComp :type Primitive%20Component%20Object%20Reference) (OtherBodyIndex :type Integer) (bFromSweep :type Boolean) (SweepResult :type Hit%20Result%20Structure%20%28by%20ref%29))
  (bind _proceduralmesh_l_lowerarm (Variables|Default|GetProceduralMesh_L_LowerArm))
  ;[0.1795 0.6056 1] Left Upper Arm
  (if (Math|Boolean|ANDBoolean (Components|ComponentHasTag OtherComp "Slicer") (Variables|ProceduralSlicing|GetCanCutLeftUpperArm?) (not (Utilities|IsValid (Variables|Default|GetTorsoRef))))
    (bind _outprocmesh (CallFunction|ProceduralMeshSliceandHide OtherComp (Variables|Default|GetProceduralMesh_L_UpperArm) (Variables|Default|GetFallOffDir_LUA) "clavicle_l" "upperarm_l"))
    (CallFunction|RespawnCharacter)
    (Utilities|IsValid _outprocmesh
      (:Is%20Valid
        (Variables|ProceduralSlicing|SetCanCutLeftUpperArm? false)
        (if (Variables|ProceduralSlicing|GetCanCutLeftLowerArm?)
          (Variables|ProceduralSlicing|SetCanCutLeftLowerArm? false)
          (Collision|SetCollisionResponsetoAllChannels _proceduralmesh_l_lowerarm "ECR_Block")
          (Collision|SetCollisionEnabled _proceduralmesh_l_lowerarm "PhysicsOnly")
          (Transformation|DetachFromComponent _proceduralmesh_l_lowerarm "KeepWorld" "KeepWorld" "KeepWorld" true)
          (Transformation|AttachComponentToComponent _proceduralmesh_l_lowerarm _outprocmesh "None" "KeepWorld" "KeepWorld" "KeepWorld" true)
          (Rendering|SetVisibility _proceduralmesh_l_lowerarm true false)
          (Transformation|SetRelativeLocationAndRotation _proceduralmesh_l_lowerarm (Variables|Default|GetRightArmRelativeLoc) (Variables|Default|GetRightArmRelativeRot) false false))))))

(event OnComponentBeginOverlap(ProceduralMesh_RLL)
  (params (OverlappedComponent :type Primitive%20Component%20Object%20Reference) (OtherActor :type Actor%20Object%20Reference) (OtherComp :type Primitive%20Component%20Object%20Reference) (OtherBodyIndex :type Integer) (bFromSweep :type Boolean) (SweepResult :type Hit%20Result%20Structure%20%28by%20ref%29))
  ;[1 0.4938 0.0916] Right LowerLeg
  (if (and (Components|ComponentHasTag OtherComp "Slicer") (Variables|ProceduralSlicing|GetCanCutRightLowerLeg?))
    (bind _outprocmesh (CallFunction|ProceduralMeshSliceandHide OtherComp (Variables|Default|GetProceduralMesh_RLL) (Variables|Default|GetFallOffDir_RLL) "thigh_r" "calf_r"))
    (Utilities|IsValid _outprocmesh
      (:Is%20Valid
        (Variables|ProceduralSlicing|SetCanCutRightLowerLeg? false)
        (CallFunction|RespawnCharacter)))))

(event OnComponentBeginOverlap(ProceduralMesh_R_UpperArm)
  (params (OverlappedComponent :type Primitive%20Component%20Object%20Reference) (OtherActor :type Actor%20Object%20Reference) (OtherComp :type Primitive%20Component%20Object%20Reference) (OtherBodyIndex :type Integer) (bFromSweep :type Boolean) (SweepResult :type Hit%20Result%20Structure%20%28by%20ref%29))
  (bind _proceduralmesh_r_lowerarm (Variables|Default|GetProceduralMesh_R_LowerArm))
  ;[0.9888 1 0.1046] Right Upper Arm
  (if (Math|Boolean|ANDBoolean (Components|ComponentHasTag OtherComp "Slicer") (Variables|ProceduralSlicing|GetCanCutRightUpperArm?) (not (Utilities|IsValid (Variables|Default|GetTorsoRef))))
    (Variables|ProceduralSlicing|SetCanCutRightUpperArm? false)
    (bind _outprocmesh (CallFunction|ProceduralMeshSliceandHide OtherComp (Variables|Default|GetProceduralMesh_R_UpperArm) (Variables|Default|GetFallOffDir_RUA) "clavicle_r" "upperarm_r"))
    (Utilities|IsValid _outprocmesh
      (:Is%20Valid
        (CallFunction|RespawnCharacter)
        (if (Variables|ProceduralSlicing|GetCanCutRightLowerArm?)
          (Variables|ProceduralSlicing|SetCanCutRightLowerArm? false)
          (Collision|SetCollisionResponsetoAllChannels _proceduralmesh_r_lowerarm "ECR_Block")
          (Collision|SetCollisionEnabled _proceduralmesh_r_lowerarm "PhysicsOnly")
          (Transformation|DetachFromComponent _proceduralmesh_r_lowerarm "KeepWorld" "KeepWorld" "KeepWorld" true)
          (Transformation|AttachComponentToComponent _proceduralmesh_r_lowerarm _outprocmesh "None" "KeepWorld" "KeepWorld" "KeepWorld" true)
          (Rendering|SetVisibility _proceduralmesh_r_lowerarm true false)
          (Transformation|SetRelativeLocationAndRotation _proceduralmesh_r_lowerarm (Variables|Default|GetRightArmRelativeLoc) (Variables|Default|GetRightArmRelativeRot) false false))))))

(event OnComponentBeginOverlap(ProceduralMesh_R_LowerArm)
  (params (OverlappedComponent :type Primitive%20Component%20Object%20Reference) (OtherActor :type Actor%20Object%20Reference) (OtherComp :type Primitive%20Component%20Object%20Reference) (OtherBodyIndex :type Integer) (bFromSweep :type Boolean) (SweepResult :type Hit%20Result%20Structure%20%28by%20ref%29))
  ;[0 1 0.3902] Right Lower Arm
  (if (Math|Boolean|ANDBoolean (Components|ComponentHasTag OtherComp "Slicer") (Variables|ProceduralSlicing|GetCanCutRightLowerArm?) (Variables|ProceduralSlicing|GetCanCutRightUpperArm?) (not (Utilities|IsValid (Variables|Default|GetTorsoRef))))
    (Variables|ProceduralSlicing|SetCanCutRightLowerArm? false)
    (CallFunction|ProceduralMeshSliceandHide OtherComp (Variables|Default|GetProceduralMesh_R_LowerArm) (Variables|Default|GetFallOffDir_RLA) "upperarm_r" "lowerarm_r")
    (CallFunction|RespawnCharacter)))

(event OnComponentBeginOverlap(ProceduralMesh_UpperLeg)
  (params (OverlappedComponent :type Primitive%20Component%20Object%20Reference) (OtherActor :type Actor%20Object%20Reference) (OtherComp :type Primitive%20Component%20Object%20Reference) (OtherBodyIndex :type Integer) (bFromSweep :type Boolean) (SweepResult :type Hit%20Result%20Structure%20%28by%20ref%29))
  (bind _proceduralmesh_rll (Variables|Default|GetProceduralMesh_RLL))
  ;[0.2814 0.1527 1] Right upper leg
  (if (and (Components|ComponentHasTag OtherComp "Slicer") (Variables|ProceduralSlicing|GetCanCutRightUpperLeg?))
    (bind _outprocmesh (CallFunction|ProceduralMeshSliceandHide OtherComp (Variables|Default|GetProceduralMesh_UpperLeg) (Variables|Default|GetFallOffDir_RUL) "pelvis" "thigh_r"))
    (Utilities|IsValid _outprocmesh
      (:Is%20Valid
        (CallFunction|RespawnCharacter)
        (Variables|ProceduralSlicing|SetCanCutRightUpperLeg? false)
        (if (Variables|ProceduralSlicing|GetCanCutRightLowerLeg?)
          (Variables|ProceduralSlicing|SetCanCutRightLowerLeg? false)
          (Collision|SetCollisionResponsetoAllChannels _proceduralmesh_rll "ECR_Block")
          (Collision|SetCollisionEnabled _proceduralmesh_rll "PhysicsOnly")
          (Transformation|DetachFromComponent _proceduralmesh_rll "KeepWorld" "KeepWorld" "KeepWorld" true)
          (Transformation|AttachComponentToComponent _proceduralmesh_rll _outprocmesh "None" "KeepWorld" "KeepWorld" "KeepWorld" true)
          (Rendering|SetVisibility _proceduralmesh_rll true false))))))

(event OnComponentBeginOverlap(ProceduralMesh_Head)
  (params (OverlappedComponent :type Primitive%20Component%20Object%20Reference) (OtherActor :type Actor%20Object%20Reference) (OtherComp :type Primitive%20Component%20Object%20Reference) (OtherBodyIndex :type Integer) (bFromSweep :type Boolean) (SweepResult :type Hit%20Result%20Structure%20%28by%20ref%29))
  ;[0.08239 0.9602 1] Head
  (if (Math|Boolean|ANDBoolean (Components|ComponentHasTag OtherComp "Slicer") (Variables|ProceduralSlicing|GetCanCutHead?) (not (Utilities|IsValid (Variables|Default|GetTorsoRef))))
    (bind _outprocmesh (CallFunction|ProceduralMeshSliceandHide OtherComp (Variables|Default|GetProceduralMesh_Head) (Variables|Default|GetFallOffDir_Head) "neck_01" "head"))
    (Utilities|IsValid _outprocmesh
      (:Is%20Valid
        (Variables|ProceduralSlicing|SetCanCutHead? false)
        (CallFunction|RespawnCharacter)))))

(event OnComponentBeginOverlap(ProceduralMesh_LLL)
  (params (OverlappedComponent :type Primitive%20Component%20Object%20Reference) (OtherActor :type Actor%20Object%20Reference) (OtherComp :type Primitive%20Component%20Object%20Reference) (OtherBodyIndex :type Integer) (bFromSweep :type Boolean) (SweepResult :type Hit%20Result%20Structure%20%28by%20ref%29))
  ;[1 0.4909 0.9935] Left lower leg
  (if (Math|Boolean|ANDBoolean (Components|ComponentHasTag OtherComp "Slicer") (Variables|ProceduralSlicing|GetCanCutLeftLowerLeg?) (Variables|ProceduralSlicing|GetCanCutLeftUpperLeg?))
    (bind _outprocmesh (CallFunction|ProceduralMeshSliceandHide OtherComp (Variables|Default|GetProceduralMesh_LLL) (Variables|Default|GetFallOffDir_LLL) "thigh_l" "calf_l"))
    (Utilities|IsValid _outprocmesh
      (:Is%20Valid
        (Variables|ProceduralSlicing|SetCanCutLeftLowerLeg? false)
        (CallFunction|RespawnCharacter)))))

(event Custom|RespawnCharacter
  ;[0 0 0] Respawn Function
  (Utilities|FlowControl|DoOnce false
    (:Completed
      (Variables|Default|SetAlive? false)
      (Actor|SetLifeSpan 5.0))))

(event EventBeginPlay
  ;[0 0 0] Comment
  (CallFunction|CreateProceduralMeshes)
  (bind _outactors (Actor|GetAllActorsOfClass "/Game/VirtualRealityBP/Blueprints/MotionControllerPawn.MotionControllerPawn_C"))
  (Variables|Default|SetPlayerRef (Utilities|Array|Get(acopy) _outactors))
  (Variables|Default|SetStartLoc (Transformation|GetActorLocation))
  (Variables|Default|SetStartRot (Transformation|GetActorRotation)))

(event EventDestroyed
  (bind _torsoref (Variables|Default|GetTorsoRef))
  ;[0 0 0] Respawn Function
  (Utilities|IsValid _torsoref
    (:Is%20Valid
      (Actor|DestroyActor _torsoref))
    (:Is%20Not%20Valid
      _))
  (bind _outactors (Actor|GetAllActorsOfClass "/Game/Blueprints/Weeb_Manager.Weeb_Manager_C"))
  (Default|RespawnDummyatLocation (Utilities|Array|Get(acopy) _outactors) (Variables|Default|GetStartLoc) (Variables|Default|GetStartRot)))

(fn ConstructionScript)

(fn GetBonestoHide
  (params (BoneHit :type Name))
  (if (Utilities|String|Contains (Utilities|String|ToString(Name) BoneHit) "spine")
    (Utilities|Array|AddUnique (LocalVariables|GetBoneList) "spine_01")
    (return (LocalVariables|GetBoneList) true)
    (else
      (switch name BoneHit
        (:lowerarm_r
          (Utilities|Array|AddUnique (LocalVariables|GetBoneList) "spine_01"))))))

(fn CanSliceBisect?
  (params (SliceLocation :type Vector) (SliceNormal :type Vector))
  (bind _horizontal_ (CallFunction|IsHorizontalSlice? SliceNormal (Math|Vector|GetForwardVector (Variables|Default|GetBisectAnchor))))
  (return (and _horizontal_ (< (.Z (Math|Vector|BreakVector SliceLocation)) (.z (Transformation|GetWorldLocation (Variables|Default|GetBisectAnchor)))))))

(fn IsHorizontalSlice?
  (params (SliceNormal :type Vector) (ComponentRightVector :type Vector))
  (return (Math|Float|InRange(Float) (Math|Float|Absolute(Float) (Class|KismetMathLibrary|DegAcos (Math|Vector|DotProduct SliceNormal ComponentRightVector))) (LocalVariables|GetMin) (LocalVariables|GetMax))))

(fn SliceinHalf
  (bind _mesh (Variables|Character|GetMesh))
  (bind _bisectanchor (Variables|Default|GetBisectAnchor))
  (Utilities|FlowControl|DoOnce false
    (:Completed
      (Variables|ProceduralSlicing|SetCanCutInHalf? false)
      (Utilities|FlowControl|Sequence
        (:then_0
          (Variables|ProceduralSlicing|SetCanCutInHalf? false)
          (Variables|ProceduralSlicing|SetCanBeCut? false))
        (:then_1
          (Components|SkinnedMesh|HideBonebyName (Variables|Character|GetMesh) "spine_01" "PBO_Term")
          (Rendering|SetVisibility (Variables|Default|GetProceduralMesh_Torso) true false))
        (:then_2
          (if (< (Math|Vector|DotProduct (Math|Vector|GetForwardVector (Variables|Default|GetFallOffDir_Torso)) (Variables|Default|GetSliceNormal)) 0.0)
            _
            (else
              (Variables|Default|SetSliceNormal (Math|Vector|NegateVector (Variables|Default|GetSliceNormal)))))
          (bind _outotherhalfprocmesh (Class|KismetProceduralMeshLibrary|SliceProceduralMesh (Variables|Default|GetProceduralMesh_Torso) (Variables|Default|GetSliceLocation) (Variables|Default|GetSliceNormal) true "CreateNewSectionForCap" "/Game/Materials/MI_GlowBlue.MI_GlowBlue"))
          (bind _output_get (Variables|Default|SetOtherHalfRef _outotherhalfprocmesh))
          (Rendering|Material|SetVectorParameterValueonMaterials _output_get "Color" (Math|Conversions|ToVector(LinearColor) (Variables|/Game/VirtualRealityBP/Blueprints/MotionControllerPawn.MotionControllerPawn_C|GetPlayerColor (Variables|Default|GetPlayerRef))))
          (Collision|SetCollisionObjectType _output_get "ECC_GameTraceChannel1")
          (Transformation|AttachComponentToComponent (Variables|Default|GetProceduralMesh_Torso) (Variables|Character|GetMesh) "pelvis" "KeepWorld" "KeepWorld" "KeepWorld" true))
        (:then_3
          ;[0 0.3375 1] Spawn Torso Upper Half
          (bind _returnvalue (Game|SpawnActorfromClass "/Game/Blueprints/Enemies/Test_Enemy_Torso_BP.Test_Enemy_Torso_BP_C" (Math|Transform|MakeTransform (Transformation|GetWorldLocation _bisectanchor) (Transformation|GetWorldRotation _bisectanchor) "1,1,1") "Undefined" 0 self 0))
          (bind _output_get_2 (Variables|Default|SetTorsoRef _returnvalue))
          (Transformation|AttachComponentToComponent (Variables|Default|GetOtherHalfRef) (Variables|/Game/Blueprints/Enemies/Test_Enemy_Torso_BP.Test_Enemy_Torso_BP_C|GetTorsoMesh _output_get_2) "spine_01" "KeepWorld" "KeepWorld" "KeepWorld" true))
        (:then_4
          ;[1 1 1] Ragdoll
          (Collision|SetCollisionEnabled _mesh "QueryAndPhysics")
          (Collision|SetCollisionResponsetoAllChannels _mesh "ECR_Block")
          (Class|SkeletalMeshComponent|SetAllBodiesSimulatePhysics _mesh true)
          (Components|DestroyComponent (Variables|Default|GetR_LowerArm)))))))

(fn FindProperSliceNormal
  (params (FallOffDirection :type Arrow%20Component%20Object%20Reference) (StartNormal :type Vector))
  (if (> (Math|Vector|DotProduct (Math|Vector|Normalize StartNormal) (Math|Vector|GetForwardVector FallOffDirection)) 0.0)
    (return (Math|Vector|NegateVector StartNormal))
    (else
      (return StartNormal))))

(fn BeginRagdoll
  (bind _mesh (Variables|Character|GetMesh))
  (Collision|SetCollisionEnabled _mesh "PhysicsOnly")
  (Collision|SetCollisionResponsetoAllChannels _mesh "ECR_Block")
  (Class|SkeletalMeshComponent|SetAllBodiesSimulatePhysics _mesh true)
  (Audio|Components|Audio|Stop _mesh))

(fn ProceduralMeshSliceandHide
  (params (HitComponent :type Primitive%20Component%20Object%20Reference) (ProceduralMesh :type Procedural%20Mesh%20Component%20Object%20Reference) (DirectionArrow :type Arrow%20Component%20Object%20Reference) (AttachBone :type Name) (HideBone :type Name))
  (bind _speed (Class|SlicerInterface|GetSpeed(Message) (Components|GetOwner HitComponent)))
  (if (> _speed (Variables|Default|GetMinCutSpeed))
    (Utilities|FlowControl|Sequence
      (:then_0
        (Variables|Default|SetSliceLocation (Transformation|GetWorldLocation HitComponent))
        (Variables|Default|SetSliceNormal (Math|Vector|GetUpVector HitComponent)))
      (:then_1
        (Transformation|AttachComponentToComponent ProceduralMesh (Variables|Character|GetMesh) AttachBone "KeepWorld" "KeepWorld" "KeepWorld" true)
        (Rendering|SetVisibility ProceduralMesh true true)
        (bind _slicenormal (CallFunction|FindProperSliceNormal DirectionArrow (Variables|Default|GetSliceNormal)))
        (bind _outotherhalfprocmesh (Class|KismetProceduralMeshLibrary|SliceProceduralMesh ProceduralMesh (Variables|Default|GetSliceLocation) _slicenormal true "CreateNewSectionForCap" "/Game/Materials/M_GlowMat.M_GlowMat"))
        (bind _output_get (LocalVariables|SetOutMeshComp _outotherhalfprocmesh))
        (Rendering|Material|SetVectorParameterValueonMaterials _output_get "Color" (Math|Conversions|ToVector(LinearColor) (Variables|/Game/VirtualRealityBP/Blueprints/MotionControllerPawn.MotionControllerPawn_C|GetPlayerColor (Variables|Default|GetPlayerRef))))
        (Collision|SetCollisionObjectType _output_get "ECC_GameTraceChannel1")
        (Collision|SetCollisionResponsetoAllChannels _output_get "ECR_Block")
        (Collision|SetCollisionEnabled _output_get "PhysicsOnly")
        (Physics|SetSimulatePhysics _output_get true)
        (Physics|AddRadialImpulse _output_get (Variables|Default|GetSliceLocation) 3e+02 5e+02 "RIF_Constant" true)
        (Variables|/Script/Engine.ActorComponent|SetComponentTags _output_get (Utilities|Array|MakeArray "SlicedBit")))
      (:then_2
        (Components|SkinnedMesh|HideBonebyName (Variables|Character|GetMesh) HideBone "PBO_Term")
        (CallFunction|BeginRagdoll))
      (:then_3
        (return (LocalVariables|GetOutMeshComp))))
    (else
      (return 0))))

(fn CreateProceduralMeshes
  (Utilities|FlowControl|Sequence
    (:then_0
      (Class|KismetProceduralMeshLibrary|CopyProceduralMeshfromStaticMeshComponent (Variables|Default|GetTorso) 0 (Variables|Default|GetProceduralMesh_Torso) true)
      (Class|KismetProceduralMeshLibrary|CopyProceduralMeshfromStaticMeshComponent (Variables|Default|GetHead) 0 (Variables|Default|GetProceduralMesh_Head) true))
    (:then_1
      (Class|KismetProceduralMeshLibrary|CopyProceduralMeshfromStaticMeshComponent (Variables|Default|GetR_LowerArm) 0 (Variables|Default|GetProceduralMesh_R_LowerArm) true)
      (Class|KismetProceduralMeshLibrary|CopyProceduralMeshfromStaticMeshComponent (Variables|Default|GetR_UpperArm) 0 (Variables|Default|GetProceduralMesh_R_UpperArm) true))
    (:then_2
      (Class|KismetProceduralMeshLibrary|CopyProceduralMeshfromStaticMeshComponent (Variables|Default|GetL_LowerArm) 0 (Variables|Default|GetProceduralMesh_L_LowerArm) true)
      (Class|KismetProceduralMeshLibrary|CopyProceduralMeshfromStaticMeshComponent (Variables|Default|GetL_UpperArm) 0 (Variables|Default|GetProceduralMesh_L_UpperArm) true))
    (:then_3
      (Class|KismetProceduralMeshLibrary|CopyProceduralMeshfromStaticMeshComponent (Variables|Default|GetR_LowerLeg) 0 (Variables|Default|GetProceduralMesh_RLL) true)
      (Class|KismetProceduralMeshLibrary|CopyProceduralMeshfromStaticMeshComponent (Variables|Default|GetR_UpperLeg) 0 (Variables|Default|GetProceduralMesh_UpperLeg) true))
    (:then_4
      (Class|KismetProceduralMeshLibrary|CopyProceduralMeshfromStaticMeshComponent (Variables|Default|GetL_LowerLeg) 0 (Variables|Default|GetProceduralMesh_LLL) true)
      (Class|KismetProceduralMeshLibrary|CopyProceduralMeshfromStaticMeshComponent (Variables|Default|GetL_UpperLeg) 0 (Variables|Default|GetProceduralMesh_LeftUpperLeg) true))))

(fn DestroyStaticMeshes
  (Utilities|FlowControl|Sequence
    (:then_0
      (Components|DestroyComponent (Variables|Default|GetTorso)))))