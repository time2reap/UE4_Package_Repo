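; VR throwable shuriken that attaches to a motion controller on pickup and launches when dropped.
; On release, it disables gravity, starts a spin mirrored for the left hand, and applies force along the unnormalized vector from the player camera to the hand's Forward component.
; A hitbox overlap while thrown stops the spin and attaches it to the hit component.
; Debug prints and lines remain, and the tracked last-frame location is unused.
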(event OnComponentBeginOverlap(Hitbox)
  (params (OverlappedComponent :type Primitive%20Component%20Object%20Reference) (OtherActor :type Actor%20Object%20Reference) (OtherComp :type Primitive%20Component%20Object%20Reference) (OtherBodyIndex :type Integer) (bFromSweep :type Boolean) (SweepResult :type Hit%20Result%20Structure%20%28by%20ref%29))
  (bind _customrotation (Variables|Default|GetCustomRotation))
  (if (Variables|Default|GetThrown?)
    (Components|Activation|SetActive _customrotation false false)
    (Variables|/Game/SP_Utility_Library/Components/CustomRotation.CustomRotation_C|SetActive _customrotation false)
    (Transformation|AttachComponentToComponent OtherComp "None" "KeepWorld" "KeepWorld" "KeepWorld" true)))

(event Custom|ThrowShuriken
  (bind _customrotation (Variables|Default|GetCustomRotation))
  (Variables|Default|SetThrown? true)
  (Development|PrintString "THROWN!" true true "(R=0.000000,G=0.233537,B=1.000000,A=1.000000)" 5.0)
  (Physics|SetEnableGravity (Variables|Default|GetVisual) false)
  (Components|Activation|SetActive (Variables|Default|GetCustomRotation) true true)
  (if (Utilities|Enum|Equal(Enum) (Variables|/Game/VirtualRealityBP/Blueprints/BP_MotionController.BP_MotionController_C|GetHand (Variables|Default|GetParentHand)) "Left")
    (Variables|/Game/SP_Utility_Library/Components/CustomRotation.CustomRotation_C|SetRotateZRate _customrotation (* (Variables|/Game/SP_Utility_Library/Components/CustomRotation.CustomRotation_C|GetRotateZRate _customrotation) -1.0)))
  (bind _direction (CallFunction|GetLaunchDirection))
  (Physics|AddForce (Variables|Default|GetVisual) (* _direction (Variables|Default|GetProjectileSpeed)) "None" false))

(event EventBeginPlay)

(event Collision|EventActorBeginOverlap
  (params (OtherActor :type Actor%20Object%20Reference)))

(event EventTick
  (params (DeltaSeconds :type Float%20%28single-precision%29))
  (Utilities|IsValid (Variables|Default|GetParentHand)
    (:Is%20Valid
      (if (not (Variables|Default|GetThrown?))
        (Variables|Default|SetLastFrameLocation (Transformation|GetActorLocation))))))

(event EventPickup
  (params (AttachTo :type Scene%20Component%20Object%20Reference))
  (bind _asbp_motion_controller (Utilities|Casting|CastToBP_MotionController (Components|GetOwner AttachTo)))
  (Variables|Default|SetParentHand _asbp_motion_controller)
  (Transformation|AttachComponentToComponent AttachTo "None" "KeepWorld" "KeepWorld" "KeepWorld" true)
  (Physics|SetSimulatePhysics (Variables|Default|GetVisual) false)
  (Transformation|SetActorRelativeLocation (Variables|Default|GetGrabLocation))
  (Transformation|SetActorRelativeRotation (Variables|Default|GetGrabRotation))
  (Variables|Default|SetThrown? false))

(event EventDrop
  (Transformation|DetachFromActor "KeepWorld" "KeepWorld" "KeepWorld")
  (Physics|SetSimulatePhysics (Variables|Default|GetVisual) true)
  (CallFunction|ThrowShuriken))

(fn ConstructionScript)

(fn GetLaunchDirection
  (bind _parenthand (Variables|Default|GetParentHand))
  (bind _forward (Variables|/Game/VirtualRealityBP/Blueprints/BP_MotionController.BP_MotionController_C|GetForward _parenthand))
  (bind _playerpawn (Variables|/Game/VirtualRealityBP/Blueprints/BP_MotionController.BP_MotionController_C|GetPlayerPawn _parenthand))
  (bind _returnvalue (Transformation|GetWorldLocation _forward))
  (bind _camera (Variables|/Game/VirtualRealityBP/Blueprints/MotionControllerPawn.MotionControllerPawn_C|GetCamera _playerpawn))
  (bind _returnvalue_2 (Transformation|GetWorldLocation _camera))
  (bind _returnvalue_3 (- _returnvalue _returnvalue_2))
  (Development|PrintString (Utilities|GetDisplayName _playerpawn) true true "(R=0.000000,G=0.660000,B=1.000000,A=1.000000)" 55.0)
  (LocalVariables|SetDirectionVector _returnvalue_3)
  (Rendering|Debug|DrawDebugLine "0, 0, 0" (+ _returnvalue_2 _returnvalue_3) (CallFunction|RandomLColorOpaque) 22.0 1.0)
  (return (LocalVariables|GetDirectionVector)))