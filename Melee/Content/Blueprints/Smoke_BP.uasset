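; Smoke actor that stays hidden until Explode, then shows a colored smoke cloud built from a sphere and particles for a set Duration.
; Explode tints the sphere materials and particles, activates SmokeScreen, and starts a timeline that scales the sphere after a short delay.
; DeathEvent stops that timeline, deactivates the spawn and persistent particles, shrinks the sphere to zero, then sets a short lifespan.
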(event Custom|PulseSmoke
  (Utilities|FlowControl|Delay 0.2)
  (bind _alpha01 (Timeline|Timeline_1 PlayFromStart)
    (:Update
      (Transformation|SetRelativeScale3D (Variables|Default|GetSphere) (Math|Vector|Lerp(Vector) (Variables|Default|GetStartScale02) (Variables|Default|GetEndScale02) _alpha01)))))

(event Custom|DeathEvent
  (Utilities|FlowControl|Sequence
    (:then_0
      (bind _alpha01 (Timeline|Timeline_1 Stop)
        (:Update
          (Transformation|SetRelativeScale3D (Variables|Default|GetSphere) (Math|Vector|Lerp(Vector) (Variables|Default|GetStartScale02) (Variables|Default|GetEndScale02) _alpha01)))))
    (:then_1
      (Components|Activation|Deactivate (Variables|Default|GetPersistentParticle))
      (bind _alpha01_2 (Timeline|Timeline_0 PlayFromStart)
        (:Update
          (Transformation|SetRelativeScale3D (Variables|Default|GetSphere) (Math|Vector|Lerp(Vector) (Variables|Default|GetStartScale02) "0, 0, 0" _alpha01_2)))
        (:Finished
          (Actor|SetLifeSpan 1.5))))))

(event Custom|Explode
  (params (Color :type Linear%20Color%20Structure))
  (CallFunction|SetColor Color)
  (Components|Activation|Activate (Variables|Default|GetSpawnParticle) true)
  (Rendering|SetVisibility (Variables|Default|GetDefaultSceneRoot) true true)
  (CallFunction|PulseSmoke)
  (Components|Activation|Activate (Variables|Default|GetSmokeScreen) true)
  (Utilities|FlowControl|Delay (Variables|Default|GetDuration))
  (CallFunction|DeathEvent))

(event EventBeginPlay
  (Rendering|SetVisibility (Variables|Default|GetDefaultSceneRoot) false true))

(fn ConstructionScript)

(fn SetColor
  (params (NewColor :type Linear%20Color%20Structure))
  (Effects|Components|ParticleSystem|SetColorParameter (Variables|Default|GetSpawnParticle) "Color" NewColor)
  (Rendering|Material|SetVectorParameterValueonMaterials (Variables|Default|GetSphere) "Color" (Math|Conversions|ToVector(LinearColor) NewColor)))