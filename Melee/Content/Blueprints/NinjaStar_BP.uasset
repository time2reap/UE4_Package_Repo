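; Thrown shuriken projectile for VR hand throwing that flies, spins and sticks to what it hits.
; BeginPlay activates projectile movement, adjusts spin and roll for the throwing hand, and applies a fixed or random color to mesh and particles.
; Tick spins the visual while thrown.
; The first valid overlap or hit, ignoring stars, bundles and controllers, attaches it, stops motion, plays effects, fades glow via timeline and sets a post-hit lifespan.
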(event OnComponentBeginOverlap(Hitbox)
  (params (OverlappedComponent :type Primitive%20Component%20Object%20Reference) (OtherActor :type Actor%20Object%20Reference) (OtherComp :type Primitive%20Component%20Object%20Reference) (OtherBodyIndex :type Integer) (bFromSweep :type Boolean) (SweepResult :type Hit%20Result%20Structure%20%28by%20ref%29))
  (bind _returnvalue (Components|GetOwner OtherComp))
  (bind _customrotation (Variables|Default|GetCustomRotation))
  (Utilities|Casting|CastToNinjaStar_BP _returnvalue
    (:CastFailed
      (Utilities|Casting|CastToBP_MotionController _returnvalue
        (:CastFailed
          (Utilities|Casting|CastToNinjaStarBundle_BP _returnvalue
            (:CastFailed
              (if (Variables|Default|GetAlive?)
                (Variables|Default|SetAlive? false)
                (Transformation|AttachComponentToComponent OtherComp "None" "KeepWorld" "KeepWorld" "KeepWorld" true)
                (Variables|/Script/Engine.MovementComponent|SetVelocity (Variables|Default|GetProjectileMovement) "0, 0, 0")
                (Variables|Default|SetThrown? false)
                (Variables|/Game/SP_Utility_Library/Components/CustomRotation.CustomRotation_C|SetActive _customrotation false)
                (Components|Activation|SetActive _customrotation false false)
                (Actor|SetLifeSpan (Variables|Default|GetLifeAfterHit))
                (Components|Activation|Deactivate (Variables|Default|GetTrailParticle))
                (Components|Activation|Activate (Variables|Default|GetHitParticle) true)
                (CallFunction|Dematerialize)
                (Audio|PlaySoundatLocation "/Game/Audio/ThrowingWeapons/ShurikenHit_Cue.ShurikenHit_Cue" (Transformation|GetWorldLocation (Variables|Default|GetVisualRoot)) "0, 0, 0" 1.0 1.0 0.0 0 0 0)))))))))

(event Custom|Dematerialize
  (bind _alpha (Timeline|Transition_TL PlayFromStart)
    (:Update
      (Rendering|Material|SetScalarParameterValueonMaterials (Variables|Default|GetVisual) "Boost" (Math|Float|Lerp 3e+02 0.0 _alpha)))))

(event EventBeginPlay
  (bind _parenthand (Variables|Default|GetParentHand))
  (bind _customrotation (Variables|Default|GetCustomRotation))
  (Actor|SetLifeSpan 3e+01)
  (Transformation|SetRelativeRotation (Variables|Default|GetVisualRoot) (Math|Rotator|MakeRotator (Math|Random|RandomFloatinRange -2e+01 2e+01) 0.0 0.0) false false)
  (Utilities|FlowControl|Sequence
    (:then_0
      ;[1 1 1] Account for hand throwing spin direction
      (Utilities|IsValid _parenthand
        (:Is%20Valid
          (switch Utilities|FlowControl|Switch|SwitchonEControllerHand (Variables|/Game/VirtualRealityBP/Blueprints/BP_MotionController.BP_MotionController_C|GetHand _parenthand)
            (:Left
              (Variables|Default|SetRotateRate (* (Variables|Default|GetRotateRate) -1.0))
              (Variables|/Game/SP_Utility_Library/Components/CustomRotation.CustomRotation_C|SetRotateXRate _customrotation (Math|Random|RandomFloatinRange -2e+01 -5.0)))
            (:Right
              (Variables|/Game/SP_Utility_Library/Components/CustomRotation.CustomRotation_C|SetRotateXRate _customrotation (Math|Random|RandomFloatinRange 5.0 2e+01)))))))
    (:then_1
      (CallFunction|SetStarColor))
    (:then_2
      (Components|Activation|Activate (Variables|Default|GetProjectileMovement) false))
    (:then_3
      (Actor|SetLifeSpan 15.0))))

(event Collision|EventHit
  (params (MyComp :type Primitive%20Component%20Object%20Reference) (Other :type Actor%20Object%20Reference) (OtherComp :type Primitive%20Component%20Object%20Reference) (bSelfMoved :type Boolean) (HitLocation :type Vector :default "0, 0, 0") (HitNormal :type Vector :default "0, 0, 0") (NormalImpulse :type Vector :default "0, 0, 0") (Hit :type Hit%20Result%20Structure%20%28by%20ref%29))
  (bind _returnvalue (Components|GetOwner OtherComp))
  (bind _customrotation (Variables|Default|GetCustomRotation))
  (Utilities|Casting|CastToNinjaStar_BP _returnvalue
    (:CastFailed
      (Utilities|Casting|CastToBP_MotionController _returnvalue
        (:CastFailed
          (Utilities|Casting|CastToNinjaStarBundle_BP _returnvalue
            (:CastFailed
              (if (Variables|Default|GetAlive?)
                (Variables|Default|SetAlive? false)
                (Transformation|AttachComponentToComponent OtherComp "None" "KeepWorld" "KeepWorld" "KeepWorld" true)
                (Variables|/Script/Engine.MovementComponent|SetVelocity (Variables|Default|GetProjectileMovement) "0, 0, 0")
                (Variables|Default|SetThrown? false)
                (Variables|/Game/SP_Utility_Library/Components/CustomRotation.CustomRotation_C|SetActive _customrotation false)
                (Components|Activation|SetActive _customrotation false false)
                (Actor|SetLifeSpan (Variables|Default|GetLifeAfterHit))
                (Components|Activation|Deactivate (Variables|Default|GetTrailParticle))
                (Components|Activation|Activate (Variables|Default|GetHitParticle) true)
                (CallFunction|Dematerialize)
                (Audio|PlaySoundatLocation "/Game/Audio/ThrowingWeapons/ShurikenHit_Cue.ShurikenHit_Cue" (Transformation|GetWorldLocation (Variables|Default|GetVisualRoot)) "0, 0, 0" 1.0 1.0 0.0 0 0 0)))))))))

(event EventTick
  (params (DeltaSeconds :type Float%20%28single-precision%29))
  (bind _visual (Variables|Default|GetVisual))
  (bind _relativerotation (Variables|/Script/Engine.SceneComponent|GetRelativeRotation _visual))
  (if (Variables|Default|GetThrown?)
    (Transformation|SetRelativeRotation _visual (Math|Rotator|MakeRotator (.roll _relativerotation) (.pitch _relativerotation) (+ (.yaw _relativerotation) (* DeltaSeconds (Variables|Default|GetRotateRate)))) false false)))

(fn ConstructionScript
  (Variables|/Script/Engine.ProjectileMovementComponent|SetInitialSpeed (Variables|Default|GetProjectileMovement) (Variables|Default|GetProjectileSpeed)))

(fn SetStarColor
  (bind _color (CallFunction|RandomLColor))
  (bind _visual (Variables|Default|GetVisual))
  (bind _starcolor (Variables|Default|GetStarColor))
  (bind _visual_2 (Variables|Default|GetVisual))
  (if (Variables|Default|GetRandomizeColor?)
    (Rendering|Material|SetVectorParameterValueonMaterials _visual "Color" (Math|Conversions|ToVector(LinearColor) _color))
    (Rendering|Material|SetScalarParameterValueonMaterials _visual "Boost" 3e+02)
    (Effects|Components|ParticleSystem|SetColorParameter (Variables|Default|GetTrailParticle) "Start Color" _color)
    (else
      (Rendering|Material|SetVectorParameterValueonMaterials _visual_2 "Color" (Math|Conversions|ToVector(LinearColor) _starcolor))
      (Rendering|Material|SetScalarParameterValueonMaterials _visual_2 "Boost" 3e+02)
      (Effects|Components|ParticleSystem|SetColorParameter (Variables|Default|GetTrailParticle) "Start Color" _starcolor))))