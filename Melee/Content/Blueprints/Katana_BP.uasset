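; VR katana actor that can be grabbed by a motion controller, drawn from a sheath and used to slice procedural meshes.
; Pickup attaches it to the hand with a timeline that eases it into grip orientation, or starts sheath mode if sheathed.
; In sheath mode, Tick maps hand distance to blade position, drawing it past a threshold.
; A plane overlap records the cut on entry, then slices and impulses the new half on exit.
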(event OnComponentBeginOverlap(ProceduralPlane)
  (params (OverlappedComponent :type Primitive%20Component%20Object%20Reference) (OtherActor :type Actor%20Object%20Reference) (OtherComp :type Primitive%20Component%20Object%20Reference) (OtherBodyIndex :type Integer) (bFromSweep :type Boolean) (SweepResult :type Hit%20Result%20Structure%20%28by%20ref%29))
  (bind _proceduralplane (Variables|Default|GetProceduralPlane))
  ;[1 0.277 0.7133] Procedural Mesh Slicing
  (if (Variables|Default|GetCanCut?)
    (Utilities|Casting|CastToProceduralMeshComponent OtherComp)
    (Utilities|FlowControl|DoOnce false
      (:Completed
        (Variables|Default|SetSlicedActor OtherActor)
        (Variables|Default|SetSlicePosition (Transformation|GetWorldLocation _proceduralplane))
        (Variables|Default|SetSliceNormal (Math|Vector|GetUpVector _proceduralplane))))))

(event OnComponentEndOverlap(ProceduralPlane)
  (params (OverlappedComponent :type Primitive%20Component%20Object%20Reference) (OtherActor :type Actor%20Object%20Reference) (OtherComp :type Primitive%20Component%20Object%20Reference) (OtherBodyIndex :type Integer))
  (bind _proceduralplane (Variables|Default|GetProceduralPlane))
  ;[1 0.277 0.7133] Procedural Mesh Slicing
  (if (== OtherActor (Variables|Default|GetSlicedActor))
    (Utilities|FlowControl|Sequence
      (:then_0
        (Variables|Default|SetSliceCapMat (CallFunction|GetRandomSliceMat))
        (bind _outotherhalfprocmesh (Class|KismetProceduralMeshLibrary|SliceProceduralMesh (Actor|GetComponentbyClass (Variables|Default|GetSlicedActor) "/Script/ProceduralMeshComponent.ProceduralMeshComponent") (Variables|Default|GetSlicePosition) (Variables|Default|GetSliceNormal) true "CreateNewSectionForCap" "/Game/Materials/MI_GlowBlue.MI_GlowBlue"))
        (Utilities|Array|AddUnique (Variables|Default|GetSubMeshes) _outotherhalfprocmesh)
        (Rendering|Material|SetVectorParameterValueonMaterials _outotherhalfprocmesh "Color" (Math|Vector|MakeVector (Math|Random|RandomFloat) (Math|Random|RandomFloat) (Math|Random|RandomFloat)))
        (Physics|SetSimulatePhysics _outotherhalfprocmesh true)
        (Physics|AddRadialImpulse _outotherhalfprocmesh (Transformation|GetWorldLocation (Variables|Default|GetProceduralPlane)) 3e+02 5e+02 "RIF_Constant" false))
      (:then_1
        (Utilities|FlowControl|DoOnce false) ; enters at Reset
      ))))

(event Custom|ResetPickup
  ;[0 1 0.01952] Event Pickup
  (Utilities|FlowControl|DoOnce false) ; enters at Reset
)

(event Custom|OrientToHand
  (bind _magnetlocation (Variables|Orientation|GetMagnetLocation))
  (bind (_x _y _z) (Math|Vector|BreakVector _magnetlocation))
  ;[1 0.9459 0.07549] Orient to Hand
  (bind _output_get (Variables|Orientation|SetOrientStartLoc (Variables|/Script/Engine.SceneComponent|GetRelativeLocation (Variables|Default|GetMesh))))
  (Variables|Orientation|SetOrientStartRot "0, 0, 0")
  (Development|PrintString (Utilities|String|ToString(Vector) _output_get) true true "(R=1.000000,G=0.000000,B=0.744031,A=1.000000)" 22.0)
  (bind _alpha (Timeline|Orientation_TL PlayFromStart)
    (:Update
      (Transformation|SetActorRelativeRotation (Math|Rotator|Lerp(Rotator) (Variables|Orientation|GetOrientStartRot) (Variables|Orientation|GetMagnetRotation) _alpha true))
      (Transformation|SetActorRelativeLocation (Math|Vector|Lerp(Vector) (Variables|Orientation|GetOrientStartLoc) (Math|Vector|MakeVector (.X (Math|Vector|BreakVector (Variables|Orientation|GetOrientStartLoc))) _y _z) _alpha)))))

(event Custom|ResetDetachment
  (bind _parenthand (Variables|Default|GetParentHand))
  (Utilities|FlowControl|DoOnce false) ; enters at Reset
)

(event EventBeginPlay
  (Variables|Orientation|SetGripStartTransform (Transformation|GetRelativeTransform (Variables|Default|GetMesh))))

(event EventPickup
  (params (AttachTo :type Scene%20Component%20Object%20Reference))
  ;[0 1 0.01952] Event Pickup
  (Utilities|FlowControl|DoOnce false
    (:Completed
      (CallFunction|ResetDetachment)
      (Development|PrintString "EVENT PICKUP" true true "(R=0.007688,G=0.000000,B=1.000000,A=1.000000)" 8.0)
      (bind _asbp_motion_controller (Utilities|Casting|CastToBP_MotionController (Components|GetOwner AttachTo)))
      (Variables|Default|SetParentHand _asbp_motion_controller)
      (if (Variables|Default|GetSheathed?)
        (Default|StartSheathing (Variables|Default|GetSheathRef))
        (Variables|Default|SetSheathing? true)
        (else
          (Physics|SetSimulatePhysics (Variables|Default|GetMesh) false)
          (Transformation|AttachComponentToComponent AttachTo "None" "KeepWorld" "KeepWorld" "KeepWorld" true)
          (CallFunction|OrienttoHand))))))

(event EventDrop
  ;[1 0 0.01548] Event Drop
  (Utilities|FlowControl|Sequence
    (:then_0
      (Variables|Default|SetParentHand 0)
      (Variables|Default|SetCanSheath? false)
      (Utilities|Time|SetTimerbyFunctionName 0 "CanSheathCD" (Variables|Default|GetSheathCD_Duration))
      (if (Variables|Default|GetSheathing?)
        (Variables|Default|SetSheathing? false)
        (if (> (Variables|Default|GetPercentUnSheathed) 45.0)
          (Variables|Default|SetSheathed? false :!label _label)
          (Variables|Default|SetPercentUnSheathed 1.0)
          (Default|StopSheathing (Variables|Default|GetSheathRef))
          (Transformation|DetachFromActor "KeepWorld" "KeepWorld" "KeepWorld")
          (Physics|SetSimulatePhysics (Variables|Default|GetMesh) false)
          (else
            (Variables|Default|SetSheathed? true)
            (Variables|Default|SetPercentUnSheathed 0.0)
            (Transformation|AttachComponentToComponent (Variables|/Game/Blueprints/Sheath_BP.Sheath_BP_C|GetSheath (Variables|Default|GetSheathRef)) "None" "KeepWorld" "KeepWorld" "KeepWorld" true)
            (CallFunction|MoveKatanainSheath (Variables|Default|GetPercentUnSheathed))
            (Default|StopSheathing (Variables|Default|GetSheathRef))))
        (else
          (goto _label))))
    (:then_1
      (CallFunction|ResetPickup))))

(event EventTick
  (params (DeltaSeconds :type Float%20%28single-precision%29))
  (bind _sheathref (Variables|Default|GetSheathRef))
  (bind _parenthand (Variables|Default|GetParentHand))
  (Utilities|FlowControl|Sequence
    (:then_0
      (if (Variables|Default|GetSheathing?)
        (bind _distance (CallFunction|CheckHandDisttoHilt))
        (if (< _distance (Variables|Default|GetMaxHandDistance))
          (bind _percentunsheathed_ (CallFunction|CalculatePercentSheathed))
          (bind _output_get (Variables|Default|SetPercentUnSheathed _percentunsheathed_))
          ;[0.2193 0.237 1] If already sheathed, remove the blade and orient in hand
          (if (and (> _output_get 0.9) (Variables|Default|GetCanDraw?))
            (Default|StopSheathing (Variables|Default|GetSheathRef))
            (Variables|Default|SetSheathed? false)
            (Variables|Default|SetSheathing? false)
            (Variables|/Game/Blueprints/Sheath_BP.Sheath_BP_C|SetSheathing? _sheathref false)
            (Default|ResetGrabAttach _sheathref)
            (Variables|Default|SetCanSheath? false)
            (Utilities|Time|SetTimerbyFunctionName 0 "CanSheathCD" (Variables|Default|GetSheathCD_Duration))
            (Audio|PlaySoundatLocation "/Game/Audio/Katana_Draw_Sching.Katana_Draw_Sching" (Transformation|GetActorLocation) "0, 0, 0" 1.0 1.0 0.0 0 0 0)
            (Physics|SetSimulatePhysics (Variables|Default|GetMesh) false)
            (Transformation|AttachComponentToComponent (Variables|Default|GetKatana_Root) (Variables|/Game/VirtualRealityBP/Blueprints/BP_MotionController.BP_MotionController_C|GetMotionController (Variables|Default|GetParentHand)) "None" "KeepWorld" "KeepWorld" "KeepWorld" true)
            (CallFunction|OrienttoHand)
            (else
              (CallFunction|MoveKatanainSheath (Variables|Default|GetPercentUnSheathed))
              (if (Variables|Default|GetSheathed?)
                (Variables|Default|SetCanDraw? true)
                (elif (< _output_get 0.65)
                  (Variables|Default|SetCanDraw? true)))))
          (else
            (Utilities|FlowControl|DoOnce false
              (:Completed
                (Variables|Default|SetSheathing? false)
                (if (> (Variables|Default|GetPercentUnSheathed) 45.0)
                  (Variables|Default|SetSheathed? false)
                  (Variables|Default|SetPercentUnSheathed 1.0)
                  (Default|StopSheathing (Variables|Default|GetSheathRef))
                  (Utilities|IsValid _parenthand
                    (:Is%20Valid
                      (CallFunction|Pickup (Variables|/Game/VirtualRealityBP/Blueprints/BP_MotionController.BP_MotionController_C|GetMotionController _parenthand))))
                  (else
                    (Variables|Default|SetSheathed? true)
                    (Variables|Default|SetPercentUnSheathed 0.0)
                    (CallFunction|MoveKatanainSheath (Variables|Default|GetPercentUnSheathed))
                    (Default|StopSheathing (Variables|Default|GetSheathRef))))))))))))

(event Custom|CanSheathCD
  (Variables|Default|SetCanSheath? true)
  (Development|PrintString "CAN SHEATH"))

(fn ConstructionScript)

(fn CalculatePercentSheathed
  (Utilities|IsValid (Variables|Default|GetSheathRef)
    (:Is%20Valid
      _)
    (:Is%20Not%20Valid
      (bind _outactors (Actor|GetAllActorsOfClass "/Game/Blueprints/Sheath_BP.Sheath_BP_C"))
      (if (Utilities|Array|IsValidIndex _outactors)
        (Variables|Default|SetSheathRef (Utilities|Array|Get(acopy) _outactors))
        (else
          (return -1.0)))))
  (return (Math|Float|Clamp(Float) (/ (CallFunction|GetDistancetoPoint (Transformation|GetWorldLocation (Variables|/Game/VirtualRealityBP/Blueprints/BP_MotionController.BP_MotionController_C|GetMotionController (Variables|Default|GetParentHand))) (Transformation|GetWorldLocation (Variables|/Game/Blueprints/Sheath_BP.Sheath_BP_C|GetHandSocket (Variables|Default|GetSheathRef))) false true false 0.0) (LocalVariables|GetHandMaxDistance)))))

(fn CheckHandDisttoHilt
  (bind _parenthand (Variables|Default|GetParentHand))
  (Utilities|IsValid _parenthand
    (:Is%20Valid
      (return (CallFunction|GetDistancetoPoint (Transformation|GetWorldLocation (Variables|Default|GetGripCenter)) (Transformation|GetWorldLocation (Variables|/Game/VirtualRealityBP/Blueprints/BP_MotionController.BP_MotionController_C|GetMotionController _parenthand)) false true true 0.0)))
    (:Is%20Not%20Valid
      (return -1.0))))

(fn MoveKatanainSheath
  (params (PercentUnSheathed :type Float%20%28single-precision%29))
  (Development|PrintString (Utilities|String|ToString(Float) PercentUnSheathed))
  (Transformation|SetRelativeLocationAndRotation (Variables|Default|GetMesh) (Math|Vector|Lerp(Vector) (Variables|Orientation|GetSheathedLocation) (Variables|Orientation|GetUnSheathedLocation) PercentUnSheathed) (Math|Rotator|Lerp(Rotator) (Variables|Orientation|GetSheathedRotation) (Variables|Orientation|GetUnSheathedRotation) PercentUnSheathed true) false false))

(fn GetRandomSliceMat
  (bind _returnvalue (Rendering|Material|CreateDynamicMaterialInstance "/Game/Materials/M_GlowMat.M_GlowMat" "None" :!class /Script/Engine.KismetMaterialLibrary))
  (bind _output_get (LocalVariables|SetMat _returnvalue))
  (Rendering|Material|SetVectorParameterValue _output_get "Color" (CallFunction|RandomLColorOpaque) :!class /Script/Engine.MaterialInstanceDynamic)
  (return (LocalVariables|GetMat)))

(fn ResetRelativeVars
  (Transformation|SetRelativeTransform (Variables|Default|GetMesh) (Variables|Orientation|GetGripStartTransform) false false))