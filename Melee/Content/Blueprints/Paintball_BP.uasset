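; Paintball projectile actor that bounces off surfaces until it bursts into an explosion effect.
; Construction sets the projectile movement's initial speed from LaunchSpeed, and BeginPlay activates it when LaunchOnStart is set.
; On hit, CheckForBreak breaks it on a very large impulse (debug-printed), random chance or exhausted bounce limit, spawning PaintballHitExplosion_BP and destroying the ball.
; LaunchProjectile is an empty stub with disconnected velocity code.
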(event EventBeginPlay
  (if (Variables|Default|GetLaunchOnStart?)
    (Components|Activation|SetActive (Variables|Default|GetProjectileMovement) true true)))

(event Collision|EventHit
  (params (MyComp :type Primitive%20Component%20Object%20Reference) (Other :type Actor%20Object%20Reference) (OtherComp :type Primitive%20Component%20Object%20Reference) (bSelfMoved :type Boolean) (HitLocation :type Vector :default "0, 0, 0") (HitNormal :type Vector :default "0, 0, 0") (NormalImpulse :type Vector :default "0, 0, 0") (Hit :type Hit%20Result%20Structure%20%28by%20ref%29))
  (bind _break_ (CallFunction|CheckforBreak (Math|Vector|VectorLength NormalImpulse)))
  (if _break_
    (Game|SpawnActorfromClass "/Game/Blueprints/PaintballHitExplosion_BP.PaintballHitExplosion_BP_C" (Math|Transform|MakeTransform HitLocation) "Undefined" 0 0)
    (Actor|DestroyActor)))

(fn ConstructionScript
  (Variables|/Script/Engine.ProjectileMovementComponent|SetInitialSpeed (Variables|Default|GetProjectileMovement) (Variables|Default|GetLaunchSpeed)))

(fn LaunchProjectile)

(fn CheckforBreak
  (params (ImpulseSize :type Float%20%28single-precision%29))
  (if (> ImpulseSize 8e+06)
    (Development|PrintString (Utilities|String|ToString(Float) ImpulseSize) true true (CallFunction|RandomLColorOpaque))
    (return true)
    (elif (< (Variables|Default|GetBounces) (Variables|Default|GetMaxBounces))
      (if (> (Math|Random|RandomFloat) 0.72)
        (return true)
        (else
          (Math|Integer|IncrementInt (Variables|Default|GetBounces)
            (:%20%20
              (return false)))))
      (else
        (return true)))))